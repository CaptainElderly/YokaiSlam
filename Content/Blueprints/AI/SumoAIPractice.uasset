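; SumoAIPractice is a practice AI Blueprint for a sumo game that chooses its behavior in the AIRun event.
; Each run calls RunStrategy, then branches on a Danger check.
; When in danger it calls RandomStrategy with a set of three enumerated strategies; otherwise it moves towards the world origin.
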(event EventBeginPlay
  (|CallParentFunction) ; This node is disabled and will not be called.\nDrag off pins to build functionality.
)

(event EventTick
  (params (DeltaSeconds :type Float%20%28single-precision%29))
  (|CallParentFunction DeltaSeconds))

(event EventAIRun
  (Utilities|RunStrategy)
  (Utilities|Danger
    (:Yes
      (CallFunction|RandomStrategy (Utilities|Array|MakeArray "NewEnumerator0" "NewEnumerator1" "NewEnumerator6")))
    (:No
      (CallFunction|MoveTowards "0, 0, 0"))))

(fn ConstructionScript
  (|CallParentFunction))