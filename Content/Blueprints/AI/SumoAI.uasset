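; AI controller base for Sumo wrestler pawns, providing ring and enemy awareness, movement helpers and timed strategies.
; Tick calls the empty AIRun hook while the match state allows, tracks grapple stalemates and destroys the controller without a pawn.
; Situational lists weight strategies by stamina, spacing and special charge for random selection.
; A periodically rerolled Stupidity, scaled by game settings, skews danger checks, attack thresholds and the post-strategy Uhh timer.
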(event Custom|AI%20Run)

(event EventBeginPlay
  (CallFunction|RerollStupidity))

(event EventTick
  (params (DeltaSeconds :type Float%20%28single-precision%29))
  (Utilities|IsValid (Pawn|GetControlledPawn)
    (:Is%20Valid
      (Flow|ResetState)
      (if (State|ShouldRunAI)
        (CallFunction|AIRun)
        (if (State|IsStalemate)
          (Variables|Default|SetStalemateTime (+ (Variables|Default|GetStalemateTime) 1.0))
          (else
            (Variables|Default|SetStalemateTime 0.0)))
        (if (>= 0 (Math|Random|RandomIntegerinRange 0 (Math|Float|Ceil (/ 2.0 (Utilities|Time|GetWorldDeltaSeconds)))))
          (CallFunction|RerollStupidity))
        (Variables|Default|SetUhh (Math|Float|Clamp(Float) (- (Variables|Default|GetUhh) DeltaSeconds) 0.0 2.0))
        (else
          (Variables|Default|SetStalemateTime 0.0))))
    (:Is%20Not%20Valid
      (Actor|DestroyActor))))

(fn ConstructionScript)

(fn GetEnemy
  (return (Default|GetTarget (State|GetMe))))

(fn HasAdvantage
  (return (< (Default|GetDistancefromRingEdge (State|GetEnemy)) (Default|GetDistancefromRingEdge (State|GetMe)))))

(fn GetMe
  (bind _assumo (Utilities|Casting|CastToSumo (Pawn|GetControlledPawn)))
  (return _assumo))

(fn GetFreeSpace
  (bind _returnvalue (State|GetEnemy))
  (bind _returnvalue_2 (State|GetMe))
  (return (- (Math|Vector|Distance2D(Vector) (Transformation|GetActorLocation _returnvalue) (Transformation|GetActorLocation _returnvalue_2)) (+ (Components|Capsule|GetScaledCapsuleRadius (Variables|/Script/Engine.Character|GetCapsuleComponent _returnvalue)) (Components|Capsule|GetScaledCapsuleRadius (Variables|/Script/Engine.Character|GetCapsuleComponent _returnvalue_2))))))

(fn GetBestEscapeDirection
  (bind _returnvalue (State|GetMe))
  (bind _returnvalue_2 (Default|GetRingEdgeNearesttoLocal _returnvalue "0,1.000000,0.000000"))
  (bind _returnvalue_3 (Default|GetRingEdgeNearesttoLocal _returnvalue "0,-1.000000, 0"))
  (bind _returnvalue_4 (Default|GetLocalTransform _returnvalue))
  (bind _returnvalue_5 (Math|Vector|Lerp(Vector) _returnvalue_3 _returnvalue_2 0.5))
  (bind _returnvalue_6 (Math|Transform|InverseTransformDirection _returnvalue_4 _returnvalue_5))
  (bind _y (Math|Vector|BreakVector _returnvalue_6))
  (bind _returnvalue_7 (* _y -1.0))
  (if (> (Math|Float|Absolute(Float) _returnvalue_7) 1.0)
    (return (Math|Float|Sign(Float) _returnvalue_7))
    (else
      (return 0.0))))

(fn Strafe
  (params (Direction :type Float%20%28single-precision%29))
  (Default|CustomMovementInput (State|GetMe) (Math|Vector|ClampVectorSize (* (.Right (State|GetEnemyDir)) Direction) 0.0 1.0) 1.0 false))

(fn IsSafetoAttack
  (bind _returnvalue (State|GetMe))
  (return (and (or (> (+ (Default|GetDistancefromRingEdge _returnvalue) (State|GetFreeSpace)) 5e+01) (State|HasAdvantage)) (> (Variables|/Game/Blueprints/Battle/Sumo.Sumo_C|GetStamina _returnvalue) 0.0))))

(fn MoveTowards
  (params (Position :type Vector))
  (bind _returnvalue (State|GetMe))
  (bind _returnvalue_2 (Transformation|GetActorLocation _returnvalue))
  (Default|CustomMovementInput _returnvalue (Math|Vector|Normalize (* (Math|Vector|GetForwardVector (Math|Rotator|FindLookatRotation _returnvalue_2 Position)) "1.000000,1.000000,0.000000")) 1.0 false)
  (return (Math|Vector|Distance2D(Vector) _returnvalue_2 Position)))

(fn IsLosingBalance
  (return (< (Variables|/Game/Blueprints/Battle/Sumo.Sumo_C|GetBalanceSkew (State|GetMe)) -1e+01)))

(fn Approach
  (Default|CustomMovementInput (State|GetMe) (.Forward (State|GetEnemyDir)) 1.0 false))

(fn Retreat
  (Default|CustomMovementInputLocal (State|GetMe) "-1.000000,0.000000, 0" 1.0 false))

(fn CanOverpower
  (bind _returnvalue (State|GetEnemy))
  (bind _returnvalue_2 (State|GetMe))
  (bind _stamina (Variables|/Game/Blueprints/Battle/Sumo.Sumo_C|GetStamina _returnvalue_2))
  (return (Math|Boolean|ANDBoolean (< (+ (Variables|/Game/Blueprints/Battle/Sumo.Sumo_C|GetStamina _returnvalue) -1e+01) _stamina) (> _stamina 6e+01) (Variables|/Game/Blueprints/Battle/Sumo.Sumo_C|GetGrappling _returnvalue) (Variables|/Game/Blueprints/Battle/Sumo.Sumo_C|GetGrappling _returnvalue_2) (State|HasAdvantage))))

(fn IsStalemate
  (bind _returnvalue (State|GetMe))
  (bind _returnvalue_2 (State|GetEnemy))
  (return (Math|Boolean|ANDBoolean (< (Math|Vector|VectorLengthXY (+ (Variables|/Script/Engine.MovementComponent|GetVelocity (Pawn|GetMovementComponent _returnvalue)) (Variables|/Script/Engine.MovementComponent|GetVelocity (Pawn|GetMovementComponent _returnvalue_2)))) 3e+01) (Variables|/Game/Blueprints/Battle/Sumo.Sumo_C|GetGrappling _returnvalue) (Variables|/Game/Blueprints/Battle/Sumo.Sumo_C|GetGrappling _returnvalue_2))))

(fn ExecuteStrategy
  (params (Strategy :type SumoStrategy%20Enum :default "NewEnumerator0") (Time :type Float%20%28single-precision%29))
  (bind _returnvalue (Game|ConstructObjectfromClass "/Game/Blueprints/AI/ExecutedStrategy.ExecutedStrategy_C" self Strategy Time))
  (Variables|Default|SetCurrentStrategy _returnvalue))

(fn ContinueStrategy
  (bind _currentstrategy (Variables|Default|GetCurrentStrategy))
  (Utilities|IsValid _currentstrategy
    (:Is%20Valid
      (bind _output_get (Variables|/Game/Blueprints/AI/ExecutedStrategy.ExecutedStrategy_C|SetTime _currentstrategy (- (Variables|/Game/Blueprints/AI/ExecutedStrategy.ExecutedStrategy_C|GetTime _currentstrategy) (Utilities|Time|GetWorldDeltaSeconds))))
      (if (<= _output_get 0.0)
        (CallFunction|FinishStrategy)
        (else
          (CallFunction|DoStrategy))))))

(fn DoStrategy
  (bind _returnvalue (State|GetBestEscapeDirection))
  (bind _returnvalue_2 (State|GetBestEscapeDirection))
  (bind _returnvalue_3 (State|GetMe))
  (bind _currentstrategy (Variables|Default|GetCurrentStrategy))
  (bind _grappling (Variables|/Game/Blueprints/Battle/Sumo.Sumo_C|GetGrappling _returnvalue_3))
  (Utilities|IsValid _currentstrategy
    (:Is%20Valid
      (switch Utilities|FlowControl|Switch|SwitchonSumoStrategy (Variables|/Game/Blueprints/AI/ExecutedStrategy.ExecutedStrategy_C|GetStrategy _currentstrategy)
        (:NewEnumerator0
          (MovementActions|Strafe -1.0)
          (if (State|IsinDanger) :!label _label
            (CallFunction|FinishStrategy)))
        (:NewEnumerator1
          (MovementActions|Strafe 1.0)
          (goto _label))
        (:NewEnumerator2
          (CallFunction|SetPushHard true)
          (Flow|Approach)
          (if (< (Variables|/Game/Blueprints/Battle/Sumo.Sumo_C|GetStamina _returnvalue_3) 2e+01)
            (CallFunction|FinishStrategy)))
        (:NewEnumerator3
          (if (Default|CanSlap _returnvalue_3)
            (if _grappling
              (Default|AIActionSlap _returnvalue_3)
              (else
                (Flow|Approach)))
            (else
              (CallFunction|FinishStrategy))))
        (:NewEnumerator5
          (if _grappling
            (if (> (Default|GetDistancefromRingEdge (State|GetMe)) 1e+02)
              (CallFunction|SetPushHard true)
              (Flow|Retreat)
              (else
                (CallFunction|FinishStrategy)))
            (else
              (Flow|Approach))))
        (:NewEnumerator6
          (MovementActions|Strafe _returnvalue)
          (if (== _returnvalue 0.0)
            (CallFunction|FinishStrategy)))
        (:NewEnumerator8
          (if (> (Default|GetDistancefromRingEdge (State|GetMe)) 2e+02)
            (Flow|Retreat)
            (elif (!= _returnvalue_2 0.0)
              (MovementActions|Strafe _returnvalue_2)
              (else
                (MovementActions|Strafe 1.0)))))
        (:NewEnumerator7
          (Default|AIRunSpecial (State|GetMe))
          (CallFunction|FinishStrategy))))))

(fn FinishStrategy
  (Variables|Default|SetCurrentStrategy 0)
  (for _index (range 0 (Variables|Default|GetStupidity))
    (if (Math|Random|RandomBool)
      (Variables|Default|SetUhh (+ (Variables|Default|GetUhh) 0.1)))))

(fn HasStrategy
  (return (Utilities|IsValid (Variables|Default|GetCurrentStrategy))))

(fn IsinDanger
  (if (> (Variables|Default|GetStupidity) 10)
    (return false)
    (else
      (return (or (Math|Boolean|ANDBoolean (< (Default|GetDistancefromRingEdge (State|GetMe)) (CallFunction|GetDangerDistance)) (not (State|HasAdvantage)) (not (or (>= (State|GetFreeSpace) 1e+02) (> (Variables|Default|GetStupidity) 0)))) (and (Variables|/Game/Blueprints/Battle/Sumo.Sumo_C|GetGrappling (State|GetMe)) (State|IsLosingBalance)))))))

(fn RandomStrategy
  (params (Choices :type Array%20of%20SumoStrategy%20Enums :default "NewEnumerator0"))
  (Utilities|Array|Shuffle Choices)
  (Utilities|Array|Shuffle Choices)
  (Utilities|Array|Shuffle Choices)
  (CallFunction|ExecuteStrategy (Utilities|Array|Get(acopy) Choices) (Math|Random|RandomFloatinRange 0.2 2.0)))

(fn HasSpecial
  (return (>= (Default|GetSpecial (State|GetMe)) 1e+02)))

(fn ShouldRunAI
  (bind _returnvalue (Pawn|GetControlledPawn))
  (if (Utilities|Enum|Equal(Enum) (CallFunction|GetMatchStatus) "NewEnumerator0")
    (Utilities|IsValid _returnvalue
      (:Is%20Valid
        (Utilities|Casting|CastToSumo _returnvalue
          (:then
            (return true))
          (:CastFailed
            _)))
      (:Is%20Not%20Valid
        _)))
  (return false))

(fn ResetState
  (Utilities|IsValid (Pawn|GetControlledPawn)
    (:Is%20Valid
      (Variables|/Game/Blueprints/Battle/Sumo.Sumo_C|SetPushHard (State|GetMe) false))
    (:Is%20Not%20Valid
      (Actor|DestroyActor))))

(fn AttemptGainAdvantage
  (bind _returnvalue (State|GetBestEscapeDirection))
  (if (!= _returnvalue 0.0)
    (MovementActions|Strafe _returnvalue)
    (return true)
    (else
      (return false))))

(fn SetPushHard
  (params (PushHard :type Boolean))
  (Variables|/Game/Blueprints/Battle/Sumo.Sumo_C|SetPushHard (State|GetMe) PushHard))

(fn GenericStrategyList
  (bind _array (Utilities|Array|MakeArray "NewEnumerator0" "NewEnumerator1" "NewEnumerator2" "NewEnumerator3" "NewEnumerator5" "NewEnumerator6"))
  (if (State|HasSpecial)
    (Utilities|Array|Add _array "NewEnumerator7"))
  (return _array))

(fn SpecialAttackAdditive
  (bind _stratlist (LocalVariables|GetStratList))
  (if (State|HasSpecial)
    (for _index (range 1 (Math|Random|RandomIntegerinRange 0 5))
      (Utilities|Array|Add _stratlist "NewEnumerator7")))
  (return _stratlist))

(fn AppendStrategyList
  (params (List1 :type Array%20of%20SumoStrategy%20Enums :default "NewEnumerator0") (List2 :type Array%20of%20SumoStrategy%20Enums :default "NewEnumerator0"))
  (Utilities|Array|AppendArray List1 List2)
  (return List1))

(fn GetDefensiveStrategies
  (bind _returnvalue (State|GetFreeSpace))
  (bind _returnvalue_2 (State|GetMe))
  (bind _returnvalue_3 (CallFunction|AddStrategyConditional (Utilities|Array|MakeArray "NewEnumerator0" "NewEnumerator1" "NewEnumerator6" "NewEnumerator8") "NewEnumerator2" (and (> (Variables|/Game/Blueprints/Battle/Sumo.Sumo_C|GetStamina _returnvalue_2) (Math|Random|RandomFloatinRange 3e+01 1e+02)) (not (Default|IsExhausted _returnvalue_2))) 1))
  (bind _returnvalue_4 (CallFunction|AddStrategyConditional _returnvalue_3 "NewEnumerator7" (State|HasSpecial) 5))
  (bind _returnvalue_5 (CallFunction|AddStrategyConditional _returnvalue_4 "NewEnumerator3" (> _returnvalue 1.5e+02) (Variables|Default|GetSlapWeight)))
  (bind _returnvalue_6 (CallFunction|AddStrategyConditional _returnvalue_5 "NewEnumerator5" (> _returnvalue 1e+02) 1))
  (return _returnvalue_6))

(fn AddStrategyConditional
  (params (List :type Array%20of%20SumoStrategy%20Enums :default "NewEnumerator0") (Strategy :type SumoStrategy%20Enum :default "NewEnumerator0") (Condition :type Boolean) (Weight :type Integer))
  (for _index (range 1 Weight)
    (if Condition
      (Utilities|Array|Add List Strategy)))
  (return List))

(fn GetOffensiveStrategies
  (bind _returnvalue (Math|Random|RandomFloatinRange 3e+01 1e+02))
  (bind _returnvalue_2 (State|GetMe))
  (bind _stupidity (Variables|Default|GetStupidity))
  (bind _returnvalue_3 (> _stupidity 3))
  (bind _returnvalue_4 (Default|IsExhausted _returnvalue_2))
  (bind _stamina (Variables|/Game/Blueprints/Battle/Sumo.Sumo_C|GetStamina _returnvalue_2))
  (bind _returnvalue_5 (not _returnvalue_4))
  (bind _returnvalue_6 (select _returnvalue_3 3.0 _returnvalue))
  (bind _returnvalue_7 (> _stamina _returnvalue_6))
  (bind _returnvalue_8 (and _returnvalue_7 _returnvalue_5))
  (bind _returnvalue_9 (CallFunction|AddStrategyConditional (Utilities|Array|MakeArray "NewEnumerator0" "NewEnumerator1" "NewEnumerator5" "NewEnumerator6" "NewEnumerator8") "NewEnumerator7" (State|HasSpecial) (select (> (Variables|Default|GetStupidity) 5) 1 3)))
  (bind _returnvalue_10 (CallFunction|AddStrategyConditional _returnvalue_9 "NewEnumerator3" (and (Default|CanSlap _returnvalue_2) _returnvalue_8) (Variables|Default|GetSlapWeight)))
  (bind _returnvalue_11 (CallFunction|AddStrategyConditional _returnvalue_10 "NewEnumerator2" _returnvalue_8 1))
  (return _returnvalue_11))

(fn GetDangerDistance
  (return (* (Math|Float|MakeLiteralFloat 1.8e+02) (/ 1.0 (Variables|/Game/Blueprints/Battle/Sumo.Sumo_C|GetWeightMul (State|GetMe))) (/ 1.0 (Variables|/Game/Blueprints/Battle/Sumo.Sumo_C|GetStrengthMul (State|GetEnemy))) (select (> (Variables|Default|GetStupidity) 1) 0.5 1.0))))

(fn GetPanicStrategies
  (bind _returnvalue (State|GetMe))
  (bind _returnvalue_2 (CallFunction|AddStrategyConditional (Utilities|Array|MakeArray "NewEnumerator8" "NewEnumerator6" "NewEnumerator0") "NewEnumerator2" (and (> (Variables|/Game/Blueprints/Battle/Sumo.Sumo_C|GetStamina _returnvalue) (Math|Random|RandomFloatinRange 7e+01 1e+02)) (not (Default|IsExhausted _returnvalue))) 1))
  (return _returnvalue_2))

(fn RerollStupidity
  (Variables|Default|SetStupidity 0)
  (for _index (range 1 (Default|GetAIStupidity (CallFunction|GetSumoGameInstance)))
    (if (== (Math|Random|RandomIntegerinRange 0 1) 0)
      (Math|Integer|IncrementInt (Variables|Default|GetStupidity)))))

(fn GetStamina
  (bind _returnvalue (State|GetMe))
  (Utilities|IsValid _returnvalue
    (:Is%20Valid
      (return (Variables|/Game/Blueprints/Battle/Sumo.Sumo_C|GetStamina _returnvalue)))
    (:Is%20Not%20Valid
      (return 0.0))))

(fn GetEnemyDir
  (bind _returnvalue (State|GetMe))
  (bind _returnvalue_2 (Default|GetTarget _returnvalue))
  (bind _returnvalue_3 (Transformation|GetActorLocation _returnvalue))
  (bind _returnvalue_4 (Transformation|GetActorLocation _returnvalue_2))
  (bind _returnvalue_5 (Math|Rotator|FindLookatRotation _returnvalue_3 _returnvalue_4))
  (return (Math|Vector|GetForwardVector _returnvalue_5) (Math|Vector|GetRightVector _returnvalue_5)))