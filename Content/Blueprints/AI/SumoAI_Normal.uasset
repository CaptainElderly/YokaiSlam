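; Normal sumo wrestler AI, likely one difficulty level, that picks strategies on each AIRun from the match situation.
; Losing balance interrupts the current strategy for a brief reaction strategy.
; Otherwise it runs the current strategy, then uses chance and thinking checks to choose random panic, offensive or defensive ones for danger, winning or neither.
; Most paths fall back to approaching and pushing hard when stamina allows; a Debug function visualises danger distance.
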(event EventBeginPlay
  (|CallParentFunction) ; This node is disabled and will not be called.\nDrag off pins to build functionality.
)

(event EventTick
  (params (DeltaSeconds :type Float%20%28single-precision%29))
  (|CallParentFunction DeltaSeconds))

(event EventAIRun
  (Utilities|LosingBalance
    (:Yes
      (Utilities|IsRunningStrategy "NewEnumerator5"
        (:Yes
          (Utilities|RunStrategy :!label _label)
          (Utilities|Danger
            (:Yes
              (Utilities|Maybe 3
                (:Yes
                  (Utilities|IsThinking
                    (:Head%20Full
                      (CallFunction|RandomStrategy (CallFunction|GetPanicStrategies)))
                    (:Head%20Empty
                      ;[1 1 1] Fallback activity when no strategy is active
                      (CallFunction|Approach :!label _label_2)
                      (Utilities|HasStaminaforResisting
                        (:Yes
                          (CallFunction|SetPushHard true))))))
                (:No
                  (goto _label_2))))
            (:No
              (Utilities|Winning
                (:Yes
                  (Utilities|Maybe 3
                    (:Yes
                      _)
                    (:No
                      (Utilities|IsBored
                        (:Yes
                          _)
                        (:No
                          (goto _label_2)))))
                  (Utilities|IsThinking
                    (:Head%20Full
                      (CallFunction|RandomStrategy (CallFunction|GetOffensiveStrategies))
                      (goto _label_2))
                    (:Head%20Empty
                      (goto _label_2))))
                (:No
                  (Utilities|IsThinking
                    (:Head%20Full
                      (Utilities|Maybe 3
                        (:Yes
                          (CallFunction|RandomStrategy (CallFunction|GetDefensiveStrategies))
                          (goto _label_2))
                        (:No
                          (goto _label_2))))
                    (:Head%20Empty
                      (goto _label_2))))))))
        (:No
          (CallFunction|FinishStrategy)
          (Utilities|IsThinking
            (:Head%20Full
              (CallFunction|ExecuteStrategy "NewEnumerator5" 0.3)
              (goto _label_2))))))
    (:No
      (goto _label))))

(fn ConstructionScript
  (|CallParentFunction))

(fn Debug
  (bind _dangerdistance (CallFunction|GetDangerDistance))
  (bind _returnvalue (- 227.5 _dangerdistance))
  (Development|PrintString (Utilities|String|ToString(Float) _returnvalue) true true "(R=0.000000,G=0.660000,B=1.000000,A=1.000000)" 0.0)
  (Rendering|Debug|DrawDebugSphere "0, 0, 0" _returnvalue 32 "(R=0.000000,G=0.484150,B=0.718750,A=1.000000)" 0.0 3.0))