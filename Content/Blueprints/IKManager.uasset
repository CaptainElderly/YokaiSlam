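; Component for the Sumo character that procedurally computes left and right foot positions for stepping.
; Each tick the active foot chases a hip-based target shifted by input, balance skew and leg split, clamped to a travel radius and pushed clear of the other foot.
; Feet swap when the planted one leaves its radius, or on a timer at low speed.
; Interpolated Z lifts the stepping foot while moving and lowers the other.
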(event EventBeginPlay
  (Variables|Default|SetFootL (* (.WorldSpace (CallFunction|GetCenterPosition false)) "1.000000,1.000000,0.000000"))
  (Variables|Default|SetFootR (* (.WorldSpace (CallFunction|GetCenterPosition true)) "1.000000,1.000000,0.000000")))

(event EventTick
  (params (DeltaSeconds :type Float%20%28single-precision%29))
  (bind _footr (Variables|Default|GetFootR))
  (bind _footl (Variables|Default|GetFootL))
  (bind _isrightfoot (Variables|Default|GetIsRightFoot))
  (bind _returnvalue (select _isrightfoot _footl _footr))
  (bind _returnvalue_2 (select _isrightfoot _footr _footl))
  (CallFunction|DebugDraw)
  (CallFunction|AddFootPosition DeltaSeconds)
  (CallFunction|FootCollision)
  (CallFunction|IdleToggle DeltaSeconds)
  (|SetBy-RefVar _returnvalue_2 (CallFunction|SetVectorZ _returnvalue_2 (Math|Interpolation|FInterpTo (CallFunction|GetVectorZ _returnvalue_2) (select (> (Math|Vector|VectorLengthXY (Variables|/Script/Engine.MovementComponent|GetVelocity (Variables|/Script/Engine.Character|GetCharacterMovement (CallFunction|GetCharacter)))) 1e+02) (Variables|Default|GetLiftHeight) 0.0) DeltaSeconds 5.0)))
  (|SetBy-RefVar _returnvalue (CallFunction|SetVectorZ _returnvalue (Math|Interpolation|FInterpTo (CallFunction|GetVectorZ _returnvalue) 0.0 DeltaSeconds 5.0))))

(fn GetFootDesiredSide)

(fn GetCenterPosition
  (params (Right :type Boolean))
  (bind _returnvalue (CallFunction|GetCharacter))
  (bind _legsplit (Variables|Default|GetLegSplit))
  (bind _capsulecomponent (Variables|/Script/Engine.Character|GetCapsuleComponent _returnvalue))
  (bind _returnvalue_2 (Transformation|GetWorldTransform _capsulecomponent))
  (bind _assumo (Utilities|Casting|CastToSumo _returnvalue))
  (return (+ (Transformation|GetSocketLocation _capsulecomponent (select Right (Variables|Default|GetHipBoneR) (Variables|Default|GetHipBoneL))) (* (CallFunction|GetFootMovementDirection) (Variables|Default|GetForwardDistance)) (Math|Transform|TransformDirection _returnvalue_2 (select Right (Math|Vector|MakeVector (+ (* (Variables|/Game/Blueprints/Battle/Sumo.Sumo_C|GetBalanceSkew _assumo) (select (Variables|/Game/Blueprints/Battle/Sumo.Sumo_C|GetGrappling _assumo) 1.0 -1.0)) (Variables|Default|GetExtraOffset)) (* _legsplit 1.0) 0.0) (Math|Vector|MakeVector (+ (* (Variables|/Game/Blueprints/Battle/Sumo.Sumo_C|GetBalanceSkew _assumo) (select (Variables|/Game/Blueprints/Battle/Sumo.Sumo_C|GetGrappling _assumo) 1.0 -1.0)) (Variables|Default|GetExtraOffset)) (* _legsplit -1.0) 0.0)))) (Math|Transform|InverseTransformLocation _returnvalue_2 (+ (Transformation|GetSocketLocation _capsulecomponent (select Right (Variables|Default|GetHipBoneR) (Variables|Default|GetHipBoneL))) (* (CallFunction|GetFootMovementDirection) (Variables|Default|GetForwardDistance)) (Math|Transform|TransformDirection _returnvalue_2 (select Right (Math|Vector|MakeVector (+ (* (Variables|/Game/Blueprints/Battle/Sumo.Sumo_C|GetBalanceSkew _assumo) (select (Variables|/Game/Blueprints/Battle/Sumo.Sumo_C|GetGrappling _assumo) 1.0 -1.0)) (Variables|Default|GetExtraOffset)) (* _legsplit 1.0) 0.0) (Math|Vector|MakeVector (+ (* (Variables|/Game/Blueprints/Battle/Sumo.Sumo_C|GetBalanceSkew _assumo) (select (Variables|/Game/Blueprints/Battle/Sumo.Sumo_C|GetGrappling _assumo) 1.0 -1.0)) (Variables|Default|GetExtraOffset)) (* _legsplit -1.0) 0.0)))))))

(fn GetMesh
  (bind _ascharacter (Utilities|Casting|CastToCharacter (Components|GetOwner)))
  (return (Variables|/Script/Engine.Character|GetMesh _ascharacter)))

(fn GetCharacter
  (bind _ascharacter (Utilities|Casting|CastToCharacter (Components|GetOwner)))
  (return _ascharacter))

(fn DebugDraw)

(fn GetFootMovementDirection
  (bind _ascharacter (Utilities|Casting|CastToCharacter (Components|GetOwner)))
  (return (Pawn|Components|PawnMovement|GetLastInputVector (Pawn|GetMovementComponent _ascharacter))))

(fn AddFootPosition
  (params (DeltaTime :type Float%20%28single-precision%29))
  (bind _footl (Variables|Default|GetFootL))
  (bind _isrightfoot (Variables|Default|GetIsRightFoot))
  (bind _footr (Variables|Default|GetFootR))
  (bind _footr_2 (Variables|Default|GetFootR))
  (bind _isrightfoot_2 (Variables|Default|GetIsRightFoot))
  (bind _isrightfoot_3 (Variables|Default|GetIsRightFoot))
  (bind _footl_2 (Variables|Default|GetFootL))
  (bind _worldspace (CallFunction|GetCenterPosition _isrightfoot))
  (bind _returnvalue (not _isrightfoot_3))
  (bind _returnvalue_2 (select _isrightfoot _footr _footl))
  (bind _returnvalue_3 (select _isrightfoot_2 _footr_2 _footl_2))
  (bind _returnvalue_4 (- _worldspace _returnvalue_2))
  (|SetBy-RefVar _returnvalue_3 (.ReturnValue (CallFunction|ClampFeet _isrightfoot_2 (+ _returnvalue_3 (* (+ (* (* (Class|KismetMathLibrary|VectorNormal2D _returnvalue_4 0.0001) (Math|Float|Clamp(Float) (/ (Math|Vector|VectorLengthXY _returnvalue_4) 5e+01))) 2e+02) (* (Variables|/Script/Engine.MovementComponent|GetVelocity (Variables|/Script/Engine.Character|GetCharacterMovement (CallFunction|GetCharacter))) (Variables|Default|GetFootChaseRate))) DeltaTime)))))
  (if (.WasOutside (CallFunction|ClampFeet _returnvalue (select _returnvalue (Variables|Default|GetFootR) (Variables|Default|GetFootL))))
    (CallFunction|SwapFoot)))

(fn ClampFeet
  (params (Right :type Boolean) (Transform :type Vector))
  (bind _worldspace (CallFunction|GetCenterPosition Right))
  (bind _mesh (CallFunction|GetMesh))
  (bind _foottravelradius (Variables|Default|GetFootTravelRadius))
  (bind _returnvalue (Transformation|GetWorldTransform _mesh))
  (bind (_location _rotation _scale) (Math|Transform|BreakTransform _returnvalue))
  (bind _returnvalue_2 (Math|Transform|MakeTransform _worldspace _rotation _scale))
  (bind _returnvalue_3 (Math|Transform|InverseTransformLocation _returnvalue_2 Transform))
  (bind _returnvalue_4 (Math|Vector|VectorClampSize2D _returnvalue_3 0.0 _foottravelradius))
  (return (Math|Transform|TransformLocation _returnvalue_2 _returnvalue_4) (Math|Vector|NotEqual(Vector) _returnvalue_3 _returnvalue_4 0.0001)))

(fn GetNextFoot)

(fn SwapFoot
  (Variables|Default|SetIsRightFoot (not (Variables|Default|GetIsRightFoot))))

(fn GetFrontmostFoot)

(fn AdjustVertical)

(fn IdleToggle
  (params (B :type Float%20%28single-precision%29))
  (if (< (Math|Vector|VectorLengthXY (Variables|/Script/Engine.MovementComponent|GetVelocity (Variables|/Script/Engine.Character|GetCharacterMovement (CallFunction|GetCharacter)))) 1e+02)
    (bind _output_get (Variables|Default|SetIdleTimer (+ (Variables|Default|GetIdleTimer) B)))
    (if (> _output_get 0.3)
      (CallFunction|SwapFoot)
      (Variables|Default|SetIdleTimer 0.0))
    (else
      (Variables|Default|SetIdleTimer 0.0))))

(fn SetVectorZ
  (params (InVector :type Vector%20%28by%20ref%29) (Z :type Float%20%28single-precision%29))
  (bind (_x _y) (Math|Vector|BreakVector InVector))
  (return (Math|Vector|MakeVector _x _y Z)))

(fn GetVectorZ
  (params (InTransform :type Vector%20%28by%20ref%29))
  (return (.Z (Math|Vector|BreakVector InTransform))))

(fn DistanceBetweenFeet
  (return (Math|Vector|Distance2D(Vector) (Variables|Default|GetFootL) (Variables|Default|GetFootR))))

(fn FootCollision
  (bind _isrightfoot (Variables|Default|GetIsRightFoot))
  (bind _footl (Variables|Default|GetFootL))
  (bind _footr (Variables|Default|GetFootR))
  (bind _minfootdistance (Variables|Default|GetMinFootDistance))
  (bind _returnvalue (select _isrightfoot _footl _footr))
  (bind _returnvalue_2 (select _isrightfoot _footr _footl))
  (bind _returnvalue_3 (- _returnvalue_2 _returnvalue))
  (if (< (CallFunction|DistanceBetweenFeet) _minfootdistance)
    (|SetBy-RefVar _returnvalue_2 (+ _returnvalue_2 (* (Class|KismetMathLibrary|VectorNormal2D _returnvalue_3 0.0001) (- _minfootdistance (Math|Vector|VectorLengthXY _returnvalue_3)))))))