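; CoinCapture is an actor that films an animated mesh, a coin going by the asset name, through a scene capture component.
; On BeginPlay it restricts SceneCaptureComponent2D to show only its StaticMesh, isolating it from the rest of the level.
; Each Tick sets the mesh's relative roll from a sine of game time, so it rocks back and forth once per second.
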(event EventBeginPlay
  (Rendering|SceneCapture|ShowOnlyComponent (Variables|Default|GetSceneCaptureComponent2D) (Variables|Default|GetStaticMesh)))

(event Collision|EventActorBeginOverlap
  (params (OtherActor :type Actor%20Object%20Reference)))

(event EventTick
  (params (DeltaSeconds :type Float%20%28single-precision%29))
  (Transformation|SetRelativeRotation (Variables|Default|GetStaticMesh) (Math|Rotator|MakeRotator (* (Math|Trig|Sin(Degrees) (* (Utilities|Time|GetGameTimeinSeconds) 3.6e+02)) 25.0) 0.0 0.0) false false))

(fn ConstructionScript)