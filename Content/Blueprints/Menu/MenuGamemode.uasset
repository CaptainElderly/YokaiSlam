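; Menu game mode for a sumo game that starts demo mode from the main menu and spawns character previews.
; Tick accumulates idle time while the master controller's current menu is MainMenu, triggers demo mode after a short delay, then pushes the timer far negative.
; RefreshCharacterPreviews replaces tagged preview Sumo actors with each planned-match player's character and skin, spread evenly in a row.
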(event EventBeginPlay)

(event EventTick
  (params (DeltaSeconds :type Float%20%28single-precision%29))
  (if (CallFunction|IsIdle)
    (bind _output_get (Variables|Default|SetIdleTime (+ (Variables|Default|GetIdleTime) DeltaSeconds)))
    (if (>= _output_get 1e+01)
      (Variables|Default|SetIdleTime -5e+02)
      (Default|StartDemoMode (CallFunction|GetSumoGameInstance)))
    (else
      (Variables|Default|SetIdleTime 0.0))))

(event EventPostLogin
  (params (NewPlayer :type Player%20Controller%20Object%20Reference)))

(fn ConstructionScript)

(fn IsIdle
  (Utilities|Casting|CastToMainMenu (Variables|/Game/Blueprints/Base/SumoBasePlayerController.SumoBasePlayerController_C|GetCurrentMenu (CallFunction|GetMasterController))
    (:then
      (return true))
    (:CastFailed
      (return false))))

(fn RefreshCharacterPreviews
  (bind _returnvalue (CallFunction|GetSumoGameInstance))
  (bind _plannedmatch (Variables|/Game/Blueprints/Base/SumoGameInstance.SumoGameInstance_C|GetPlannedMatch _returnvalue))
  (bind _players (Utilities|Struct|BreakMatchSettings _plannedmatch))
  (bind _outactors (Actor|GetAllActorsOfClasswithTag "/Game/Blueprints/Battle/Sumo.Sumo_C" "PreviewObject"))
  (for _array_element _outactors
    (Actor|DestroyActor _array_element))
  (for (_ _array_index) _players
    (if (Utilities|IsValidClass (.Character (Utilities|Struct|BreakCharacterSelection (CallFunction|GetCharacter _plannedmatch _array_index))))
      (bind _returnvalue_2 (Game|SpawnActorfromClass (.Character (Utilities|Struct|BreakCharacterSelection (CallFunction|GetCharacter _plannedmatch _array_index))) (Math|Transform|MakeTransform (Math|Vector|MakeVector 3e+02 (Math|Float|MapRangeClamped (Math|Conversions|ToFloat(Integer) _array_index) 0.0 (Math|Conversions|ToFloat(Integer) (- (Utilities|Array|Length _players) 1)) -2e+02 2e+02) 1e+02) "0,180.000000, 0") "AlwaysSpawn" 0 _array_index 0))
      (Utilities|Array|Add (Variables|/Script/Engine.Actor|GetTags _returnvalue_2) "PreviewObject")
      (Variables|/Game/Blueprints/Battle/Sumo.Sumo_C|SetAlternateMaterialIndex _returnvalue_2 (.Skin (Utilities|Struct|BreakCharacterSelection (CallFunction|GetCharacter _plannedmatch _array_index))))
      (Default|HandleAlternateSkin _returnvalue_2))))