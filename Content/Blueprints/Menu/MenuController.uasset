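; Player controller for the game's menus, which opens the screen stored in the game instance's next menu state.
; On possess or begin play it briefly waits, fades the camera in, resets game state when heading to the main menu, opens that widget and rebuilds character previews.
; Remote clients check every tick to steer their menu to character select.
; Input drops the keyboard token or resets the gamemode's idle timer.
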(event EventBeginPlay
  (bind _returnvalue (CallFunction|GetSumoGameInstance))
  (Utilities|FlowControl|Delay 0.1)
  (CameraFades|StartCameraFade :self (Game|GetPlayerCameraManager 0) :FromAlpha 1.0 :Duration 1.0 :bShouldFadeAudio (Variables|/Game/Blueprints/Base/SumoGameInstance.SumoGameInstance_C|GetFadeIn (CallFunction|GetSumoGameInstance)))
  (if (== (Variables|/Game/Blueprints/Base/SumoGameInstance.SumoGameInstance_C|GetNextMenuState _returnvalue) "/Game/Blueprints/Menu/MainMenu.MainMenu_C")
    (Default|ResetGameState (CallFunction|GetSumoGameInstance)))
  (Default|OpenWidget (CallFunction|GetMasterController) (Variables|/Game/Blueprints/Base/SumoGameInstance.SumoGameInstance_C|GetNextMenuState (CallFunction|GetSumoGameInstance)))
  (Default|RebuildCharacterPreviews _returnvalue))

(event EventTick
  (params (DeltaSeconds :type Float%20%28single-precision%29))
  (|CallParentFunction DeltaSeconds)
  (Networking|SwitchHasAuthority
    (:Remote
      (CallFunction|GetTargetClientMenu))))

(event EventPossess
  (params (PossessedPawn :type Pawn%20Object%20Reference))
  (bind _returnvalue (CallFunction|GetSumoGameInstance))
  (Utilities|FlowControl|Delay 0.1)
  (CameraFades|StartCameraFade :self (Game|GetPlayerCameraManager 0) :FromAlpha 1.0 :Duration 1.0 :bShouldFadeAudio (Variables|/Game/Blueprints/Base/SumoGameInstance.SumoGameInstance_C|GetFadeIn (CallFunction|GetSumoGameInstance)))
  (if (== (Variables|/Game/Blueprints/Base/SumoGameInstance.SumoGameInstance_C|GetNextMenuState _returnvalue) "/Game/Blueprints/Menu/MainMenu.MainMenu_C")
    (Default|ResetGameState (CallFunction|GetSumoGameInstance)))
  (Default|OpenWidget (CallFunction|GetMasterController) (Variables|/Game/Blueprints/Base/SumoGameInstance.SumoGameInstance_C|GetNextMenuState (CallFunction|GetSumoGameInstance)))
  (Default|RebuildCharacterPreviews _returnvalue))

(event Input|ActionEvents|InputActionSlap
  (params (Key :type Key%20Structure :default "None"))
  (:Pressed
    (Default|DropKeyboard (Variables|Default|GetToken))))

(event Input|KeyboardEvents|Period
  (params (Key :type Key%20Structure :default "None"))
  (:Pressed
    (Development|PrintString "I was going to make this key lead to a secret kappa fight but that crashed the game and i ran out of time. Perhaps next time :^)")))

(event Input|KeyboardEvents|AnyKey
  (params (Key :type Key%20Structure :default "None"))
  (:Pressed
    (Variables|/Game/Blueprints/Menu/MenuGamemode.MenuGamemode_C|SetIdleTime (CallFunction|GetMenuGamemode) 0.0)))

(fn ConstructionScript)

(fn GetTargetClientMenu
  (bind _returnvalue (select true "/Game/Blueprints/Menu/CharacterSelect.CharacterSelect_C" 0))
  (bind _currentmenu (Variables|Default|GetCurrentMenu))
  (bind _returnvalue_2 (Utilities|GetClass _currentmenu))
  (if (CallFunction|IsClient)
    (Utilities|IsValid _currentmenu
      (:Is%20Valid
        (if (!= _returnvalue_2 _returnvalue)
          (if (Utilities|IsValidClass _returnvalue_2)
            (CallFunction|OpenWidget _returnvalue :!label _label)
            (Variables|/Game/Blueprints/Base/SumoGameInstance.SumoGameInstance_C|SetNextMenuState (CallFunction|GetSumoGameInstance) _returnvalue)
            (else
              (CallFunction|DestroyWidget)))))
      (:Is%20Not%20Valid
        (goto _label)))))

(fn MoveToken
  (params (NewParam :type Vector%202D%20Structure)))