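; Menu preview actor that shows the sumo character chosen for its slot in the planned match.
; Rebuild, run on BeginPlay, resets and hides the mesh, then applies the mesh, animation class, scale and skin material from the character's class defaults.
; Bodies from the upper-body bone down simulate physics over the animation.
; Tick jitters the mesh's relative location by a tiny random offset every frame.
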(event Custom|Rebuild
  (bind _returnvalue (CallFunction|GetSumoGameInstance))
  (bind _skeletalmesh (Variables|Default|GetSkeletalMesh))
  (bind _skeletalmesh_2 (Variables|Default|GetSkeletalMesh))
  (bind _choiceindex (Variables|Default|GetChoiceIndex))
  (bind _plannedmatch (Variables|/Game/Blueprints/Base/SumoGameInstance.SumoGameInstance_C|GetPlannedMatch _returnvalue))
  (bind _returnvalue_2 (CallFunction|GetCharacter _plannedmatch _choiceindex))
  (bind _skin (Utilities|Struct|BreakCharacterSelection _returnvalue_2))
  (bind (_preview_mesh _preview_anim _preview_scale _valid _upper_body_bone _skins _alternate_material_index) (CallFunction|GetSumo))
  (CallFunction|ResetBody)
  (if _valid
    (Utilities|FlowControl|Delay 0.0)
    (Components|Animation|SetAnimationMode _skeletalmesh_2 "AnimationBlueprint")
    (Class|SkinnedMeshComponent|SetSkeletalMesh _skeletalmesh_2 _preview_mesh true)
    (Class|SkeletalMeshComponent|SetAnimClass _skeletalmesh_2 _preview_anim)
    (Transformation|SetWorldScale3D _skeletalmesh_2 (Math|Conversions|ToVector(Float) _preview_scale))
    (Utilities|FlowControl|Delay 0.0)
    (Rendering|SetVisibility _skeletalmesh_2 true false)
    (Components|SkinnedMesh|SetPhysicsAsset _skeletalmesh (Variables|/Script/Engine.SkeletalMesh|GetPhysicsAsset _preview_mesh) true)
    (Class|SkeletalMeshComponent|ResetAllBodiesSimulatePhysics _skeletalmesh)
    (Class|SkeletalMeshComponent|SetAllBodiesBelowSimulatePhysics _skeletalmesh _upper_body_bone true true)
    (if (Utilities|Array|IsValidIndex _skins _skin)
      (Rendering|Material|SetMaterial _skeletalmesh_2 _alternate_material_index (Utilities|Array|Get(acopy) _skins _skin))
      (else
        (Rendering|Material|SetMaterial (Variables|Default|GetSkeletalMesh) _alternate_material_index 0)))))

(event EventBeginPlay
  (CallFunction|Rebuild))

(event Collision|EventActorBeginOverlap
  (params (OtherActor :type Actor%20Object%20Reference)))

(event EventTick
  (params (DeltaSeconds :type Float%20%28single-precision%29))
  (Transformation|SetRelativeLocation (Variables|Default|GetSkeletalMesh) (* (Math|Random|RandomUnitVector) 0.1) false false))

(fn ConstructionScript)

(fn GetSumo
  (bind _returnvalue (CallFunction|GetSumoGameInstance))
  (bind _choiceindex (Variables|Default|GetChoiceIndex))
  (bind _plannedmatch (Variables|/Game/Blueprints/Base/SumoGameInstance.SumoGameInstance_C|GetPlannedMatch _returnvalue))
  (bind _returnvalue_2 (CallFunction|GetCharacter _plannedmatch _choiceindex))
  (bind _character (Utilities|Struct|BreakCharacterSelection _returnvalue_2))
  (bind (_previewmesh _previewanim _previewscale _unlockflag _upperbodybone _skins _alternatematerialindex) (Utilities|GetClassDefaults _character))
  (if (Utilities|IsValidClass _character)
    (return _previewmesh _previewanim _previewscale true _upperbodybone _skins _alternatematerialindex)
    (else
      (return "/Engine/EditorMeshes/SkeletalMesh/DefaultSkeletalMesh.DefaultSkeletalMesh" "/Script/Engine.AnimInstance" 1.0 false "None" (Utilities|Array|MakeArray) 0))))

(fn ResetBody
  (bind _skeletalmesh (Variables|Default|GetSkeletalMesh))
  (bind _skeletalmesh_2 (Variables|Default|GetSkeletalMesh))
  (Class|SkinnedMeshComponent|SetSkeletalMesh _skeletalmesh_2 0 true)
  (Class|SkeletalMeshComponent|SetAnimClass _skeletalmesh_2)
  (Rendering|SetVisibility _skeletalmesh_2 false false)
  (Physics|SetSimulatePhysics _skeletalmesh false)
  (Class|SkeletalMeshComponent|SetAnimClass _skeletalmesh)
  (Components|Animation|SetAnimationMode _skeletalmesh "AnimationBlueprint")
  (Components|SkinnedMesh|SetPhysicsAsset _skeletalmesh 0 true))