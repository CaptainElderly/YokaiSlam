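; Game instance for the sumo game, holding state that outlives level loads: save data, unlocks, settings, music and the planned match.
; Init functions build PlannedMatch per mode, which EnterGame opens after a camera fade, using servertravel on online servers.
; Unlock flags, AI stupidity and graphics levels persist in one save slot; data tables map graphics options to console commands and define cheat codes.
; Match setup is server-gated through IgnoreForClient.
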(event Custom|EnterGame
  (params (Duration :type Float%20%28single-precision%29) (bShouldFadeAudio :type Boolean))
  (bind _plannedmatch (Variables|Default|GetPlannedMatch))
  (bind (_targetmap _targetgamemode) (Utilities|Struct|BreakMatchSettings _plannedmatch))
  (Utilities|IgnoreforClient)
  (CameraFades|StartCameraFade :self (Game|GetPlayerCameraManager 0) :ToAlpha 1.0 :Duration Duration :bShouldFadeAudio bShouldFadeAudio :bHoldWhenFinished true)
  (Utilities|FlowControl|Delay Duration)
  (CallFunction|EnterMap _targetmap _targetgamemode)
  (Default|DestroyWidget (CallFunction|GetMasterController)))

(event Custom|EnterMenu
  (params (NextMenuState :type User%20Widget%20Class%20Reference) (FadeTime :type Float%20%28single-precision%29) (StayInGame :type Boolean) (ForceReset :type Boolean) (bShouldFadeAudio :type Boolean))
  (bind _returnvalue (CallFunction|GetMenuGamemode))
  (Variables|SumoGameInstance_C|SetNextMenuState self NextMenuState)
  (if ForceReset
    (CameraFades|StartCameraFade :self (Game|GetPlayerCameraManager 0) :ToAlpha 1.0 :Duration FadeTime :bShouldFadeAudio bShouldFadeAudio :bHoldWhenFinished true :!label _label)
    (Utilities|FlowControl|Delay FadeTime)
    (Variables|Default|SetFadeIn bShouldFadeAudio)
    (Game|OpenLevel(byName) "Menu")
    (else
      (bind _returnvalue_2 (Game|GetCurrentLevelName true))
      (if (Utilities|Enum|Equal(Enum) _returnvalue_2 "Menu")
        (Default|OpenWidget (CallFunction|GetMasterController) NextMenuState)
        (Utilities|IsValid _returnvalue
          (:Is%20Valid
            (Default|ClearCharacterPreviews _returnvalue)))
        (elif StayInGame
          (Default|OpenWidget (CallFunction|GetMasterController) NextMenuState)
          (else
            (goto _label)))))))

(event Custom|ClearTournament
  (Utilities|IgnoreforClient))

(event Custom|StartDemoMode
  (Utilities|IgnoreforClient)
  (GameTypes|InitDemoMode)
  (CallFunction|EnterGame 0.2 false))

(event Custom|CheatEntered
  (params (Cheat :type Name) (On :type Boolean))
  (switch name Cheat
    (:UnlockAll
      (CallFunction|SetUnlockFlag "AlternateSkins" true)
      (CallFunction|SetUnlockFlag "Maps" true)
      (for _array_element (Variables|Default|GetAllCharacters)
        (CallFunction|UnlockCharacter _array_element)))
    (:Terrible
      (GameTypes|InitTerrible)
      (CallFunction|EnterGame 0.1 true))))

(event Custom|EndDemoMode
  (Utilities|IgnoreforClient)
  (CallFunction|EnterMenu "/Game/Blueprints/Menu/MainMenu.MainMenu_C" 0.2 false true false)
  (CallFunction|ResetGameState))

(event Custom|DestroyMenu
  (Default|DestroyWidget (CallFunction|GetMasterController)))

(event EventInit
  (CallFunction|Load)
  (bind _returnvalue (Game|GetCurrentLevelName true))
  (if (Utilities|Enum|NotEqual(Enum) _returnvalue "Menu")
    _))

(fn UnlockCharacter
  (params (Character :type Sumo%20Class%20Reference))
  (bind _unlockflag (Utilities|GetClassDefaults Character))
  (if (and (CallFunction|IsCharacterLocked Character) (Utilities|Name|NotEqual(Name) _unlockflag "None"))
    (CallFunction|SetUnlockFlag _unlockflag true)
    (CallFunction|Save)))

(fn GetPlayerColor
  (params (ID :type Integer))
  (bind _playercolors (Variables|Default|GetPlayerColors))
  (if (Utilities|Array|IsValidIndex _playercolors ID)
    (return (Utilities|Array|Get(acopy) _playercolors ID))
    (else
      (return "(R=1.000000,G=0.000000,B=0.873395,A=1.000000)"))))

(fn IsCharacterLocked
  (params (Character :type Sumo%20Class%20Reference))
  (bind _unlockflag (Utilities|GetClassDefaults Character))
  (return (and (Utilities|Name|NotEqual(Name) _unlockflag "None") (not (Utilities|Set|Contains (Variables|/Game/Blueprints/Base/SumoSaveGame.SumoSaveGame_C|GetUnlockFlags (Variables|Default|GetSaveObject)) _unlockflag)))))

(fn GetRandomLockedCharacter
  (for _array_element (Variables|Default|GetAllCharacters)
    (if (and (CallFunction|IsCharacterLocked _array_element) (!= _array_element "/Game/Blueprints/Fighters/Sumo_Ube.Sumo_Ube_C"))
      (return _array_element)))
  (return 0))

(fn GetSaveValue)

(fn Save
  (SaveGame|SaveGametoSlot (Variables|Default|GetSaveObject) "sumo")
  (CallFunction|ApplyGraphics false))

(fn Load
  (bind _returnvalue (SaveGame|DoesSaveGameExist "sumo"))
  (if _returnvalue
    (bind _returnvalue_2 (SaveGame|LoadGamefromSlot "sumo"))
    (bind _assumo_save_game (Utilities|Casting|CastToSumoSaveGame _returnvalue_2))
    (Variables|Default|SetSaveObject _assumo_save_game)
    (else
      (bind _returnvalue_3 (SaveGame|CreateSaveGameObject "/Game/Blueprints/Base/SumoSaveGame.SumoSaveGame_C"))
      (Variables|Default|SetSaveObject _returnvalue_3)))
  (CallFunction|ApplyGraphics false))

(fn ResetGameState
  (Variables|Default|SetPlannedMatch ""))

(fn GetTargetMusic
  (bind _returnvalue (Game|GetGameMode))
  (if (CallFunction|IsMusicEnabled)
    (Utilities|Casting|CastToSumoGamemode _returnvalue
      (:then
        (if (Utilities|Name|Equal(Name) (.TargetGamemode (Utilities|Struct|BreakMatchSettings (Variables|Default|GetPlannedMatch))) "Demo")
          _
          (elif true
            (return "/Game/Music/final.final")
            (else
              (return "/Game/Music/percussion_and_bass.percussion_and_bass")))))
      (:CastFailed
        (Utilities|Casting|CastToMenuGamemode _returnvalue)))
    (return "/Game/Music/ebackground.ebackground")
    (else
      (return 0))))

(fn TickMusic
  (bind _returnvalue (CallFunction|GetTargetMusic))
  (Utilities|IsValid (Variables|Default|GetCurrentMusic)
    (:Is%20Valid
      (if (!= _returnvalue (Variables|/Script/Engine.AudioComponent|GetSound (Variables|Default|GetCurrentMusic)))
        (Audio|Components|Audio|Stop (Variables|Default|GetCurrentMusic))
        (if (Utilities|IsValid _returnvalue) :!label _label
          (bind _returnvalue_2 (Audio|CreateSound2D _returnvalue 1.0 1.0 0.0 0 true))
          (bind _output_get (Variables|Default|SetCurrentMusic _returnvalue_2))
          (Audio|Components|Audio|Play _output_get 0.0))))
    (:Is%20Not%20Valid
      (goto _label)))
  (Utilities|IsValid (Variables|Default|GetCurrentMusic)
    (:Is%20Valid
      (Audio|Components|Audio|SetVolumeMultiplier (Variables|Default|GetCurrentMusic) (select (Game|IsGamePaused) 0.2 0.5) :!class /Script/Engine.AudioComponent))))

(fn ApplyGraphics
  (params (Initial :type Boolean))
  (bind _returnvalue (Game|GetPlayerController 0))
  (bind _outrownames (DataTable|GetDataTableRowNames "/Game/Blueprints/Setting/Settings.Settings"))
  (for _array_element _outrownames
    (bind _returnvalue_2 (Utilities|GetDataTableRow "/Game/Blueprints/Setting/Settings.Settings" _array_element)
      (:then
        (if (.ReturnValue (Utilities|Map|Find (Variables|/Game/Blueprints/Base/SumoSaveGame.SumoSaveGame_C|GetGraphicsLevels (Variables|Default|GetSaveObject)) _array_element))
          (if (and (Class|GameplayStatics|HasLaunchOption "-safemode") Initial)
            (if (Utilities|Array|IsEmpty (.ConsoleVar (Utilities|Struct|BreakSettingDefinition _returnvalue_2))) :!label _label
              _
              (else
                (Development|ExecuteConsoleCommand (CallFunction|CommandHandling (.ConsoleVar (Utilities|Struct|BreakSettingDefinition _returnvalue_2)) (Utilities|Array|Get(acopy) (.Options (Utilities|Struct|BreakSettingDefinition _returnvalue_2)) (.DefaultOption (Utilities|Struct|BreakSettingDefinition _returnvalue_2)))) _returnvalue)))
            (LocalVariables|SetSetValue (Utilities|Array|Get(acopy) (.Options (Utilities|Struct|BreakSettingDefinition _returnvalue_2)) (.DefaultOption (Utilities|Struct|BreakSettingDefinition _returnvalue_2))))
            (else
              (if (Utilities|Array|IsEmpty (.ConsoleVar (Utilities|Struct|BreakSettingDefinition _returnvalue_2)))
                _
                (else
                  (Development|ExecuteConsoleCommand (CallFunction|CommandHandling (.ConsoleVar (Utilities|Struct|BreakSettingDefinition _returnvalue_2)) (Utilities|Array|Get(acopy) (.Options (Utilities|Struct|BreakSettingDefinition _returnvalue_2)) (.Value (Utilities|Map|Find (Variables|/Game/Blueprints/Base/SumoSaveGame.SumoSaveGame_C|GetGraphicsLevels (Variables|Default|GetSaveObject)) _array_element)))) _returnvalue)))
              (LocalVariables|SetSetValue (Utilities|Array|Get(acopy) (.Options (Utilities|Struct|BreakSettingDefinition _returnvalue_2)) (.Value (Utilities|Map|Find (Variables|/Game/Blueprints/Base/SumoSaveGame.SumoSaveGame_C|GetGraphicsLevels (Variables|Default|GetSaveObject)) _array_element))))))
          (else
            (goto _label))))
      (:RowNotFound
        (goto _label)))
    (switch name _array_element)))

(fn SetGraphicsSetting
  (params (Type :type Name) (Value :type Integer))
  (bind _returnvalue (Utilities|GetDataTableRow "/Game/Blueprints/Setting/Settings.Settings" Type)
    (:then
      (if (Utilities|Array|IsValidIndex (.Options (Utilities|Struct|BreakSettingDefinition _returnvalue)) Value)
        (Utilities|Map|Add (Variables|/Game/Blueprints/Base/SumoSaveGame.SumoSaveGame_C|GetGraphicsLevels (Variables|Default|GetSaveObject)) Type Value)
        (CallFunction|Save)))))

(fn GetGraphicsSetting
  (params (Type :type Name))
  (bind _saveobject (Variables|Default|GetSaveObject))
  (bind _graphicslevels (Variables|/Game/Blueprints/Base/SumoSaveGame.SumoSaveGame_C|GetGraphicsLevels _saveobject))
  (bind (_value _returnvalue) (Utilities|Map|Find _graphicslevels Type))
  (if _returnvalue
    (return _value)
    (else
      (bind _returnvalue_2 (Utilities|GetDataTableRow "/Game/Blueprints/Setting/Settings.Settings" Type)
        (:then
          (return (.DefaultOption (Utilities|Struct|BreakSettingDefinition _returnvalue_2))))
        (:RowNotFound
          (Development|PrintString "BIG ERROR! Requesting unknown setting index")
          (return 0))))))

(fn AddGraphicsValue
  (params (Type :type Name) (Offset :type Integer))
  (bind _returnvalue (Utilities|GetDataTableRow "/Game/Blueprints/Setting/Settings.Settings" Type)
    (:then
      (bind _output_get (LocalVariables|SetTargetValue (+ (CallFunction|GetGraphicsSetting Type) Offset)))
      (if (< _output_get 0)
        (LocalVariables|SetTargetValue (- (Utilities|Array|Length (.Options (Utilities|Struct|BreakSettingDefinition _returnvalue))) 1))
        (elif (> _output_get (- (Utilities|Array|Length (.Options (Utilities|Struct|BreakSettingDefinition _returnvalue))) 1))
          (LocalVariables|SetTargetValue 0)))
      (CallFunction|SetGraphicsSetting Type (LocalVariables|GetTargetValue)))))

(fn CommandHandling
  (params (Command :type String) (Value :type String))
  (switch string Command
    (:Default
      (return (Utilities|String|Append Command " " Value)))
    (:r.SetRes
      (return (Utilities|String|Append Command " " Value (Utilities|Select :Index (CallFunction|GetGraphicsSetting "ViewportMode") :Option%200 "f" :Option%201 "f" :Option%202 "w"))))))

(fn AreSkinsUnlocked
  (return (CallFunction|HasUnlockFlag "AlternateSkins")))

(fn RebuildCharacterPreviews)

(fn GetRandomCharacter
  (params (RequireUnlock :type Boolean))
  (bind _workinglist (LocalVariables|GetWorkingList))
  (for _array_element (Variables|Default|GetAllCharacters)
    (if (or (not RequireUnlock) (not (CallFunction|IsCharacterLocked _array_element)))
      (Utilities|Array|Add (LocalVariables|GetWorkingList) _array_element)))
  (return (Utilities|Array|Get(acopy) _workinglist (- (Math|Random|RandomIntegerinRange 1 (Utilities|Array|Length _workinglist)) 1))))

(fn InitTournament
  (Utilities|IgnoreforClient)
  (bind _returnvalue (CallFunction|CreateMatch "Tournament" "TournamentArena" false))
  (bind _output_get (Variables|Default|SetPlannedMatch _returnvalue))
  (return _output_get))

(fn InitTraining
  (Utilities|IgnoreforClient)
  (bind _returnvalue (CallFunction|CreateMatch "Training" "TrainingArena" false))
  (bind _output_get (Variables|Default|SetPlannedMatch _returnvalue))
  (Utilities|Array|SetArrayElem (Variables|Default|GetPlayerColors) 2 "(R=0.354167,G=0.354167,B=0.354167,A=1.000000)")
  (return _output_get))

(fn InitSingleMatch
  (Utilities|IgnoreforClient)
  (bind _returnvalue (CallFunction|CreateMatch "Default" "TournamentArena" false))
  (bind _output_get (Variables|Default|SetPlannedMatch _returnvalue))
  (if (CallFunction|AreMapsUnlocked)
    _
    (else
      (Utilities|Struct|SetmembersinMatchSettings _output_get "Maps" "You unlocked the ability to play any mode on any stage! 
Try another game to see what's available!")))
  (return _output_get))

(fn InitDemoMode
  (Utilities|IgnoreforClient)
  (bind _returnvalue (CallFunction|CreateMatch "Demo" "VoidArena" true))
  (bind _output_get (Variables|Default|SetPlannedMatch _returnvalue))
  (return _output_get))

(fn GetAIStupidity
  (return (Variables|/Game/Blueprints/Base/SumoSaveGame.SumoSaveGame_C|GetAIStupidity (Variables|Default|GetSaveObject))))

(fn SetAIStupidity
  (params (AIStupidity :type Integer))
  (Variables|/Game/Blueprints/Base/SumoSaveGame.SumoSaveGame_C|SetAIStupidity (Variables|Default|GetSaveObject) AIStupidity)
  (CallFunction|Save))

(fn AddAIStupidity
  (bind _output_get (LocalVariables|SetRunningVar (+ (CallFunction|GetAIStupidity) 1)))
  (if (> _output_get 20)
    (LocalVariables|SetRunningVar 0))
  (CallFunction|SetAIStupidity (LocalVariables|GetRunningVar)))

(fn EnterCheat
  (params (Code :type Name))
  (bind _activecheats (Variables|Default|GetActiveCheats))
  (bind _returnvalue (Utilities|GetDataTableRow "/Game/Blueprints/Base/CheatCodes.CheatCodes" Code)
    (:then
      (if (.Toggle (Utilities|Struct|BreakCheatCode _returnvalue))
        (if (Utilities|Set|Contains _activecheats Code)
          (Utilities|Set|Remove _activecheats Code)
          (CallFunction|CheatEntered Code false)
          (else
            (Utilities|Set|Add _activecheats Code)
            (CallFunction|CheatEntered Code true)))
        (else
          (CallFunction|CheatEntered Code true))))))

(fn IsCheatActive
  (params (Cheat :type Name))
  (return (Utilities|Set|Contains (Variables|Default|GetActiveCheats) Cheat)))

(fn InitTerrible
  (Utilities|IgnoreforClient)
  (bind _returnvalue (CallFunction|CreateMatch "Demo" "VoidArena" true))
  (Variables|Default|SetPlannedMatch _returnvalue)
  (CallFunction|SetPlayerTypeinSlot _returnvalue 2 "NewEnumerator3")
  (CallFunction|SetPlayerTypeinSlot _returnvalue 3 "NewEnumerator3"))

(fn ReplicateMatchState
  (Utilities|Casting|CastToMenuGameState (CallFunction|GetMasterGameState)))

(fn HasUnlockFlag
  (params (Flag :type Name))
  (return (Utilities|Set|Contains (Variables|/Game/Blueprints/Base/SumoSaveGame.SumoSaveGame_C|GetUnlockFlags (Variables|Default|GetSaveObject)) Flag)))

(fn SetUnlockFlag
  (params (Flag :type Name) (Value :type Boolean))
  (bind _saveobject (Variables|Default|GetSaveObject))
  (bind _unlockflags (Variables|/Game/Blueprints/Base/SumoSaveGame.SumoSaveGame_C|GetUnlockFlags _saveobject))
  (if Value
    (Utilities|Set|Add _unlockflags Flag)
    (else
      (Utilities|Set|Remove _unlockflags Flag)))
  (CallFunction|Save))

(fn AreMapsUnlocked
  (return (CallFunction|HasUnlockFlag "Maps")))

(fn SpecialFight
  (params (Character :type Sumo%20Class%20Reference) (Skin :type Integer))
  (bind (_unlockflag _charactername) (Utilities|GetClassDefaults Character))
  (bind _plannedmatch (Variables|Default|GetPlannedMatch))
  (GameTypes|InitSingleMatch)
  (CallFunction|SetCharacter _plannedmatch 1 (Utilities|Struct|MakeCharacterSelection Character Skin))
  (CallFunction|SetPlayerTypeinSlot _plannedmatch 1 "NewEnumerator3")
  (if (and (CallFunction|IsCharacterLocked Character) (Utilities|Name|NotEqual(Name) _unlockflag "None"))
    (Utilities|Struct|SetmembersinMatchSettings _plannedmatch _unlockflag (Utilities|Text|FormatText "You unlocked the ability to play as {cname}!" _charactername))))

(fn EnterMap
  (params (LevelName :type Name) (GamemodeName :type Name))
  (bind _returnvalue (Utilities|String|ToString(Name) GamemodeName))
  (bind _returnvalue_2 (Utilities|String|Append "game=" _returnvalue))
  (if (.ReturnValue (CallFunction|IsOnlineServer))
    (Development|ExecuteConsoleCommand (Utilities|String|Append "servertravel " (Utilities|String|ToString(Name) LevelName) "?" _returnvalue_2) (CallFunction|GetMasterController))
    (else
      (Game|OpenLevel(byName) LevelName true _returnvalue_2))))