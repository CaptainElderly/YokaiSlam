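; Blueprint function library for creating, editing and querying MatchSettings structs in a sumo fighting game.
; CreateMatch assigns player or AI slots by gamemode, while helpers set fighters and skins and check readiness.
; GenerateTournament shuffles and trims unlocked opponents excluding the player's character, then appends a finale that can offer a locked character or alternate skins as reward.
; Progress helpers advance that queue, and GiveMatchReward writes the win message and unlock flag to the game instance.
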(fn GenerateTournament
  (params (Match :type Match%20Settings%20Structure%20%28by%20ref%29) (Max%20Rounds :type Integer))
  (bind ___worldcontext (LocalVariables|Get__WorldContext))
  (bind _workingqueue (LocalVariables|GetWorkingQueue))
  (bind _workingqueue_2 (LocalVariables|GetWorkingQueue))
  (bind _returnvalue (Utilities|Array|Length _workingqueue_2))
  (bind _returnvalue_2 (CallFunction|GetSumoGameInstance ___worldcontext))
  ;[1 1 1] Layer 1. Make us a list of possible generic contenders. No locked character and none of the character you're fighting as
  (if (Utilities|Name|Equal(Name) (.TargetGamemode (Utilities|Struct|BreakMatchSettings Match)) "Tournament")
    (for _array_element (Variables|/Game/Blueprints/Base/SumoGameInstance.SumoGameInstance_C|GetAllCharacters _returnvalue_2)
      (if (and (not (Default|IsCharacterLocked _returnvalue_2 _array_element)) (!= (.Character (Utilities|Struct|BreakCharacterSelection (CallFunction|GetCharacter Match))) _array_element))
        (Utilities|Array|Add (LocalVariables|GetChoices) _array_element)))
    ;[1 1 1] Layer 2, Fill up the queue with everyone, shuffle it
    (for _array_element_2 (LocalVariables|GetChoices)
      (Utilities|Array|Add _workingqueue (Utilities|Struct|MakeCharacterSelection _array_element_2)))
    (Utilities|Array|Shuffle _workingqueue)
    ;[1 1 1] Layer 3: Trim tournment to length, and add finale content
    (bind (_character _valid _unlockflag _unlockmessage) (CallFunction|GetTournamentFinaleContent Match (LocalVariables|Get__WorldContext)))
    (for _index (range 0 _returnvalue)
      (if (> _returnvalue (- Max%20Rounds (select _valid 1 0)))
        (Utilities|Array|RemoveIndex _workingqueue_2)))
    (Utilities|Array|Add _workingqueue_2 _character)
    (Utilities|Struct|SetmembersinMatchSettings Match (LocalVariables|GetWorkingQueue) _unlockflag _unlockmessage)))

(fn GetTournamentFinaleContent
  (params (Match :type Match%20Settings%20Structure%20%28by%20ref%29))
  (bind _returnvalue (CallFunction|GetCharacter Match))
  (bind ___worldcontext (LocalVariables|Get__WorldContext))
  (bind _skinset (LocalVariables|GetSkinSet))
  (bind (_character _skin) (Utilities|Struct|BreakCharacterSelection _returnvalue))
  (bind _returnvalue_2 (CallFunction|GetSumoGameInstance ___worldcontext))
  (bind _array_element (Default|GetRandomLockedCharacter _returnvalue_2))
  (bind (_unlockflag _charactername) (Utilities|GetClassDefaults _array_element))
  (if (Utilities|IsValidClass _array_element)
    (return (Utilities|Struct|MakeCharacterSelection _array_element) true _unlockflag (Utilities|Text|FormatText "Great job! You unlocked the ability to play as the character {cname}." _charactername))
    (elif (Default|AreSkinsUnlocked _returnvalue_2)
      (return "" true "None" "")
      (else
        (Utilities|Array|RemoveItem _skinset _skin)
        (Utilities|Array|Shuffle _skinset)
        (return (Utilities|Struct|MakeCharacterSelection _character (Utilities|Array|Get(acopy) _skinset)) false "AlternateSkins" "Congratulations! You unlocked alternate skins for each character!")))))

(fn CreateMatch
  (params (TargetGamemode :type Name) (DefaultMap :type Name) (ForceDefaultMap :type Boolean))
  (bind _returnvalue (CallFunction|IsOnlineServer))
  (bind _returnvalue_2 (not ForceDefaultMap))
  (bind _returnvalue_3 (CallFunction|GetMenuGamemode))
  (bind _custommapunlocked (|CustomMapsUnlocked?))
  (bind _returnvalue_4 (and _returnvalue_2 _custommapunlocked))
  (bind _returnvalue_5 (select _returnvalue "NewEnumerator4" "NewEnumerator1"))
  (bind _returnvalue_6 (select _returnvalue_4 "None" DefaultMap))
  (bind _matchsettings (Utilities|Struct|MakeMatchSettings "NewEnumerator0" 0 _returnvalue_6 TargetGamemode 0 0 "None" "" true))
  (Utilities|FlowControl|Sequence
    (:then_0
      (switch name TargetGamemode
        (:Default
          (Match|SetPlayerTypeinSlot _matchsettings 0 _returnvalue_5 :!label _label)
          (Match|SetPlayerTypeinSlot _matchsettings 1 (select (|Arewedoinglocalmultiplayer?) _returnvalue_5 "NewEnumerator2")))
        (:Tournament
          (Match|SetPlayerTypeinSlot _matchsettings 0 "NewEnumerator1")
          (Match|SetPlayerTypeinSlot _matchsettings 1 "NewEnumerator3"))
        (:Training
          (goto _label))
        (:Demo
          (Match|SetPlayerTypeinSlot _matchsettings 0 "NewEnumerator2")
          (Match|SetPlayerTypeinSlot _matchsettings 1 "NewEnumerator2"))))
    (:then_1
      (Utilities|IsValid _returnvalue_3
        (:Is%20Valid
          (Default|RefreshCharacterPreviews _returnvalue_3))))
    (:then_2
      (return _matchsettings))))

(fn SetPlayerTypeinSlot
  (params (Match :type Match%20Settings%20Structure%20%28by%20ref%29) (Slot :type Integer) (Type :type PlayerType%20Enum :default "NewEnumerator0"))
  (Utilities|Array|SetArrayElem (.Players (Utilities|Struct|BreakMatchSettings Match)) Slot Type true))

(fn GetPlayerTypeinSlot
  (params (Match :type Match%20Settings%20Structure%20%28by%20ref%29) (Slot :type Integer))
  (bind _players (Utilities|Struct|BreakMatchSettings Match))
  (if (Utilities|Array|IsValidIndex _players Slot)
    (return (Utilities|Array|Get(acopy) _players Slot))
    (else
      (return "NewEnumerator0"))))

(fn GetCharacter
  (params (Match :type Match%20Settings%20Structure%20%28by%20ref%29) (Slot :type Integer))
  (bind _characters (Utilities|Struct|BreakMatchSettings Match))
  (if (Utilities|Array|IsValidIndex _characters Slot)
    (return (Utilities|Array|Get(acopy) _characters Slot))
    (else
      (return ""))))

(fn SetCharacter
  (params (Match :type Match%20Settings%20Structure%20%28by%20ref%29) (Index :type Integer) (Item :type Character%20Selection%20Structure%20%28by%20ref%29))
  (Utilities|Array|SetArrayElem (.Characters (Utilities|Struct|BreakMatchSettings Match)) Index Item true))

(fn ChooseFighter
  (params (Match :type Match%20Settings%20Structure%20%28by%20ref%29) (Slot :type Integer) (Character :type Sumo%20Class%20Reference))
  (CallFunction|SetCharacter Match Slot (Utilities|Struct|MakeCharacterSelection Character (.Skin (Utilities|Struct|BreakCharacterSelection (CallFunction|GetCharacter Match Slot)))))
  (Default|RefreshCharacterPreviews (CallFunction|GetMenuGamemode)))

(fn ChooseSkin
  (params (Match :type Match%20Settings%20Structure%20%28by%20ref%29) (Slot :type Integer) (Skin :type Integer))
  (CallFunction|SetCharacter Match Slot (Utilities|Struct|MakeCharacterSelection (.Character (Utilities|Struct|BreakCharacterSelection (CallFunction|GetCharacter Match Slot))) Skin)))

(fn IsReadytoStart
  (params (Match :type Match%20Settings%20Structure%20%28by%20ref%29))
  (for (_array_element _array_index) (.Players (Utilities|Struct|BreakMatchSettings Match))
    (switch Utilities|FlowControl|Switch|SwitchonPlayerType _array_element
      (:NewEnumerator1
        _)
      (:NewEnumerator4
        _)
      (:NewEnumerator2
        _))
    (if (not (CallFunction|HasCharacter Match _array_index))
      (LocalVariables|SetIsReady false)))
  (return (LocalVariables|GetIsReady)))

(fn HasCharacter
  (params (Match :type Match%20Settings%20Structure%20%28by%20ref%29) (Slot :type Integer))
  (bind _characters (Utilities|Struct|BreakMatchSettings Match))
  (if (Utilities|Array|IsValidIndex _characters Slot)
    (return (Utilities|IsValidClass (.Character (Utilities|Struct|BreakCharacterSelection (Utilities|Array|Get(acopy) _characters Slot)))))
    (else
      (return false))))

(fn IsOnline
  (params (Match :type Match%20Settings%20Structure%20%28by%20ref%29))
  (for _array_element (.Players (Utilities|Struct|BreakMatchSettings Match))
    (if (Utilities|Enum|Equal(Enum) _array_element "NewEnumerator4")
      (return true)))
  (return false))

(fn NeedstoGenerateTournament
  (params (Match :type Match%20Settings%20Structure%20%28by%20ref%29))
  (bind (_targetgamemode _tournamentqueue) (Utilities|Struct|BreakMatchSettings Match))
  (if (Utilities|Name|Equal(Name) _targetgamemode "Tournament")
    (return (== (Utilities|Array|Length _tournamentqueue) 0))
    (else
      (return false))))

(fn IsFinale
  (params (Match :type Match%20Settings%20Structure%20%28by%20ref%29))
  (bind (_players _characters _targetmap _targetgamemode _tournamentqueue _tournamentprogress) (Utilities|Struct|BreakMatchSettings Match))
  (if (Utilities|Name|Equal(Name) _targetgamemode "Tournament")
    (return (== (- (Utilities|Array|Length _tournamentqueue) 1) _tournamentprogress))
    (else
      (return false))))

(fn HasPlayer
  (params (Match :type Match%20Settings%20Structure%20%28by%20ref%29) (Slot :type Integer))
  (bind _players (Utilities|Struct|BreakMatchSettings Match))
  (if (Utilities|Array|IsValidIndex _players Slot)
    (return (Utilities|Enum|NotEqual(Enum) (Utilities|Array|Get(acopy) _players Slot) "NewEnumerator0"))
    (else
      (return false))))

(fn GetCharacterName
  (params (Match :type Match%20Settings%20Structure%20%28by%20ref%29) (Slot :type Integer))
  (bind _returnvalue (CallFunction|GetCharacter Match Slot))
  (bind _character (Utilities|Struct|BreakCharacterSelection _returnvalue))
  (if (Utilities|IsValidClass _character)
    (return (.CharacterName (Utilities|GetClassDefaults _character)))
    (else
      (return ""))))

(fn ProceedTournament
  (params (Match :type Match%20Settings%20Structure%20%28by%20ref%29))
  (bind (_players _characters _targetmap _targetgamemode _tournamentqueue _tournamentprogress) (Utilities|Struct|BreakMatchSettings Match))
  (Utilities|Struct|SetmembersinMatchSettings Match (+ _tournamentprogress 1))
  (return (not (Utilities|Array|IsValidIndex _tournamentqueue _tournamentprogress))))

(fn GiveMatchReward
  (params (Match :type Match%20Settings%20Structure%20%28by%20ref%29))
  (bind (_tournamentreward _rewardtext) (Utilities|Struct|BreakMatchSettings Match))
  (bind _returnvalue (CallFunction|GetSumoGameInstance))
  (if (CallFunction|HasReward Match)
    (Variables|/Game/Blueprints/Base/SumoGameInstance.SumoGameInstance_C|SetWinMessage _returnvalue _rewardtext)
    (Default|SetUnlockFlag _returnvalue _tournamentreward true)))

(fn HasReward
  (params (Match :type Match%20Settings%20Structure%20%28by%20ref%29))
  (return (Utilities|Name|NotEqual(Name) (.TournamentReward (Utilities|Struct|BreakMatchSettings Match)) "None")))

(fn IsValid
  (params (Match :type Match%20Settings%20Structure%20%28by%20ref%29))
  (return (Utilities|Struct|BreakMatchSettings Match)))