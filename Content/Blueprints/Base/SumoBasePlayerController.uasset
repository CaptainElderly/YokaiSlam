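; Base player controller for the Sumo game that manages the current menu widget, pausing and input focus.
; Opening a menu replaces the previous one and pauses if the game mode allows; destroying it restores game focus.
; Tick calls music updates and toggles a post-process effect for the EpicMode cheat.
; Menu replication is inactive: its server-side logic is disconnected and the client handler is empty.
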(event Custom|OpenWidget
  (params (Class :type User%20Widget%20Class%20Reference))
  ;[1 1 1] Wacky Internal stuff, no touching or overriding
  (Utilities|IsValid (Variables|Default|GetCurrentMenu)
    (:Is%20Valid
      (Widget|RemovefromParent (Variables|Default|GetCurrentMenu)))
    (:Is%20Not%20Valid
      _))
  (bind _returnvalue (UserInterface|CreateWidget Class self))
  (UserInterface|Viewport|AddtoViewport _returnvalue 0)
  (bind _output_get (Variables|Default|SetCurrentMenu _returnvalue))
  (CallFunction|FocusAllUserstoWidget _output_get)
  (Game|SetGamePaused (Variables|/Script/Engine.GameModeBase|GetbPauseable (Game|GetGameMode))))

(event Custom|FadeToMenu
  (params (Duration :type Float%20%28single-precision%29) (B :type Object%20Class%20Reference))
  (CameraFades|StartCameraFade :self (Game|GetPlayerCameraManager 0) :FromAlpha 1.0 :Duration Duration :bShouldFadeAudio true)
  (Utilities|FlowControl|Delay Duration))

(event Custom|DestroyWidget
  ;[1 1 1] Wacky Internal stuff, no touching or overriding
  (Utilities|IsValid (Variables|Default|GetCurrentMenu)
    (:Is%20Valid
      (Widget|RemovefromParent (Variables|Default|GetCurrentMenu)))
    (:Is%20Not%20Valid
      _))
  (Variables|Default|SetCurrentMenu 0)
  (CallFunction|FocusAllUserstoGame)
  (Game|SetGamePaused false))

(event EventBeginPlay)

(event EventTick
  (params (DeltaSeconds :type Float%20%28single-precision%29))
  (CallFunction|TickMusic)
  (CallFunction|ReplicateMenu)
  (CallFunction|ClientHandleMenu)
  (CallFunction|EpicMode))

(fn ConstructionScript)

(fn ReplicateMenu
  (Utilities|IsValid (CallFunction|GetMenuGameState)))

(fn ClientHandleMenu)

(fn EpicMode
  (Rendering|AddorUpdateBlendable (Variables|SumoBasePlayerController_C|GetPostProcess (CallFunction|GetMasterController)) (Variables|/Game/Blueprints/Base/SumoGameInstance.SumoGameInstance_C|GetCoolEffect (CallFunction|GetSumoGameInstance)) (select (CallFunction|IsCheatActive "EpicMode") 1.0 0.0) :!class /Script/Engine.PostProcessComponent))