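; CommonGameFunctions is a shared helper library for the Sumo game, giving global access to its game modes, states, instance and first player controller.
; Cast-based getters underpin shortcuts for match status, music and cheat checks.
; Focus helpers switch local player controllers between UI-only and game-only input, with the widget variant skipping array index 1.
; Network helpers detect an online server by counting non-local controllers and derive client status from that.
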(fn GetMatchStatus
  (bind ___worldcontext (LocalVariables|Get__WorldContext))
  (bind _returnvalue (CallFunction|GetSumoGameState ___worldcontext))
  (Utilities|IsValid _returnvalue
    (:Is%20Valid
      (return (Variables|/Game/Blueprints/Battle/SumoGameState.SumoGameState_C|GetGameStatus _returnvalue)))
    (:Is%20Not%20Valid
      (return "NewEnumerator5"))))

(fn GetSumoGamemode
  (bind _assumo_gamemode (Utilities|Casting|CastToSumoGamemode (Game|GetGameMode (LocalVariables|Get__WorldContext)))
    (:then
      (return _assumo_gamemode))
    (:CastFailed
      (return 0))))

(fn GetSumoGameInstance
  (bind _assumo_game_instance (Utilities|Casting|CastToSumoGameInstance (Game|GetGameInstance (LocalVariables|Get__WorldContext)))
    (:then
      (return _assumo_game_instance))
    (:CastFailed
      (return 0))))

(fn IsMusicEnabled
  (return (Variables|/Game/Blueprints/Base/SumoSaveGame.SumoSaveGame_C|GetMusicOn (Variables|/Game/Blueprints/Base/SumoGameInstance.SumoGameInstance_C|GetSaveObject (CallFunction|GetSumoGameInstance (LocalVariables|Get__WorldContext))))))

(fn TickMusic
  (Default|TickMusic (CallFunction|GetSumoGameInstance (LocalVariables|Get__WorldContext))))

(fn GetMenuGamemode
  (bind _asmenu_gamemode (Utilities|Casting|CastToMenuGamemode (Game|GetGameMode (LocalVariables|Get__WorldContext)))
    (:then
      (return _asmenu_gamemode))
    (:CastFailed
      (return 0))))

(fn FocusAllUserstoWidget
  (params (Widget :type Widget%20Object%20Reference))
  (bind _outactors (Actor|GetAllActorsOfClass (LocalVariables|Get__WorldContext) "/Script/Engine.PlayerController"))
  (for (_array_element _array_index) _outactors
    (Utilities|IsValid _array_element
      (:Is%20Valid
        (if (and (Pawn|IsLocalController _array_element) (!= _array_index 1))
          (Input|SetInputModeUIOnly _array_element Widget "DoNotLock")
          (Variables|/Script/Engine.PlayerController|SetbShowMouseCursor _array_element true))))))

(fn FocusAllUserstoGame
  (bind _outactors (Actor|GetAllActorsOfClass (LocalVariables|Get__WorldContext) "/Script/Engine.PlayerController"))
  (for _array_element _outactors
    (Utilities|IsValid _array_element
      (:Is%20Valid
        (if (Pawn|IsLocalController _array_element)
          (Input|SetInputModeGameOnly _array_element)
          (Variables|/Script/Engine.PlayerController|SetbShowMouseCursor _array_element false))))))

(fn IsOnlineServer
  (bind ___worldcontext (LocalVariables|Get__WorldContext))
  (if (Networking|IsServer ___worldcontext)
    (bind _outactors (Actor|GetAllActorsOfClass ___worldcontext "/Script/Engine.PlayerController"))
    (for _array_element _outactors
      (if (not (Pawn|IsLocalController _array_element))
        (LocalVariables|SetClientFound true)
        (Math|Integer|IncrementInt (LocalVariables|GetPlayerCount))))
    (return (LocalVariables|GetClientFound) (LocalVariables|GetPlayerCount))
    (else
      (return false 0))))

(fn GetSumoGameState
  (bind _assumo_game_state (Utilities|Casting|CastToSumoGameState (Game|GetGameState (LocalVariables|Get__WorldContext))))
  (return _assumo_game_state))

(fn GetMasterController
  (bind _assumo_base_player_controller (Utilities|Casting|CastToSumoBasePlayerController (Game|GetPlayerController (LocalVariables|Get__WorldContext))))
  (return _assumo_base_player_controller))

(fn IsClient
  (bind ___worldcontext (LocalVariables|Get__WorldContext))
  (return (and (not (.ReturnValue (CallFunction|IsOnlineServer ___worldcontext))) (not (Networking|IsServer ___worldcontext)))))

(fn IsCheatActive
  (params (Cheat :type Name))
  (return (Default|IsCheatActive (CallFunction|GetSumoGameInstance (LocalVariables|Get__WorldContext)) Cheat)))

(fn GetMenuGameState
  (bind _asmenu_game_state (Utilities|Casting|CastToMenuGameState (Game|GetGameState (LocalVariables|Get__WorldContext))))
  (return _asmenu_game_state))

(fn GetMasterGameState
  (bind _assumo_base_game_state (Utilities|Casting|CastToSumoBaseGameState (Game|GetGameState (LocalVariables|Get__WorldContext))))
  (return _assumo_base_game_state))