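; Game state for a sumo battle, holding the active match, player scores and shared status queries.
; On BeginPlay the authority copies the game instance's planned match, or builds a two-character Training fallback.
; AddPoint respects the gamemode's scoring switch, and three points ends the game.
; Tick respawns a missing side camera, while helpers report movement rules, singleplayer, winner and an average position of disqualified sumos.
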(event EventTick
  (params (DeltaSeconds :type Float%20%28single-precision%29))
  (CallFunction|ConfirmCamera))

(event EventBeginPlay
  (bind _returnvalue (CallFunction|GetSumoGameInstance))
  (bind _plannedmatch (Variables|/Game/Blueprints/Base/SumoGameInstance.SumoGameInstance_C|GetPlannedMatch _returnvalue))
  (|CallParentFunction)
  (Networking|SwitchHasAuthority
    (:Authority
      (if (CallFunction|IsValid _plannedmatch)
        (Variables|Default|SetActiveMatchInfo (|Copy _plannedmatch))
        (else
          (bind _returnvalue_2 (CallFunction|CreateMatch "Training" "TrainingArena" false))
          (CallFunction|SetCharacter _returnvalue_2 0 (Utilities|Struct|MakeCharacterSelection "/Game/Blueprints/Fighters/Sumo_Tsuyoi.Sumo_Tsuyoi_C" 2))
          (CallFunction|SetCharacter _returnvalue_2 1 (Utilities|Struct|MakeCharacterSelection "/Game/Blueprints/Fighters/Sumo_Glasgow.Sumo_Glasgow_C" 1))
          (Variables|Default|SetActiveMatchInfo _returnvalue_2))))))

(fn ConstructionScript)

(fn MovementRulesActive
  (return (Utilities|Enum|Equal(Enum) (Variables|Default|GetGameStatus) "NewEnumerator0")))

(fn IsGameOver
  (for _array_element (Variables|SumoGameState_C|GetScores (CallFunction|GetSumoGameState))
    (if (>= _array_element 3)
      (return true)))
  (return false))

(fn GetPlayerScore
  (params (Index :type Integer))
  (bind _scores (Variables|Default|GetScores))
  (if (Utilities|Array|IsValidIndex _scores Index)
    (return (Utilities|Array|Get(acopy) _scores Index))
    (else
      (return 0))))

(fn GetPlayerbyID
  (params (Index :type Integer))
  (bind _players (Variables|Default|GetPlayers))
  (if (Utilities|Array|IsValidIndex _players Index)
    (return (Utilities|Array|Get(acopy) _players Index))
    (else
      (return 0))))

(fn AddPoint
  (params (Player :type Integer))
  (bind _scores (Variables|Default|GetScores))
  (if (not (Variables|/Game/Blueprints/Battle/SumoGamemode.SumoGamemode_C|GetDisableScoring (CallFunction|GetSumoGamemode)))
    (if (Utilities|Array|IsValidIndex _scores Player)
      (Math|Integer|IncrementInt (Utilities|Array|Get(acopy) _scores Player))
      (else
        (Utilities|Array|SetArrayElem _scores Player 1 true)))))

(fn ConfirmCamera
  (Utilities|IsValid (Variables|Default|GetSideCamera)
    (:Is%20Not%20Valid
      (bind _returnvalue (Game|SpawnActorfromClass "/Game/Blueprints/Battle/SideCamera.SideCamera_C" (Math|Transform|MakeTransform "0, 0,100.000000") "AlwaysSpawn" self 0))
      (Variables|Default|SetSideCamera _returnvalue))))

(fn GetCenterOfGame
  (bind _positions (LocalVariables|GetPositions))
  (bind _outactors (Actor|GetAllActorsOfClass "/Game/Blueprints/Battle/Sumo.Sumo_C"))
  (if (|Aretheresumosatall?_2 _outactors)
    (for _array_element _outactors
      (if (Variables|/Game/Blueprints/Battle/Sumo.Sumo_C|GetDisqualified _array_element)
        (Utilities|Array|Add _positions (Transformation|GetActorLocation _array_element))))
    (return (Math|Vector|GetVectorArrayAverage _positions))))

(fn IsSingleplayer
  (for _array_element (.Players (Utilities|Struct|BreakMatchSettings (Variables|SumoGameState_C|GetActiveMatchInfo (CallFunction|GetSumoGameState))))
    (switch Utilities|FlowControl|Switch|SwitchonPlayerType _array_element
      (:NewEnumerator1
        (Math|Integer|IncrementInt (LocalVariables|GetPlayerCount)))))
  (return (== (LocalVariables|GetPlayerCount) 1)))

(fn IsLocalPlayerWinner
  (if (and (CallFunction|IsSingleplayer) (CallFunction|IsGameOver))
    (if (== (Variables|Default|GetWinner) 0)
      (return true)
      (else
        _)))
  (return true))