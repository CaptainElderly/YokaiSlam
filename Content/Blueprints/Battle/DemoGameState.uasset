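; DemoGameState is a battle Blueprint, apparently a game state, that owns a shared DemoCamera reference, SideCamera.
; ConfirmCamera lazily creates it: when SideCamera is invalid, it spawns a DemoCamera at a fixed spot above the world origin, owned by this actor, and stores it.
; The event graph holds only disabled default events, so nothing in this asset calls ConfirmCamera.
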(event EventBeginPlay
  (|CallParentFunction) ; This node is disabled and will not be called.\nDrag off pins to build functionality.
)

(event EventTick
  (params (DeltaSeconds :type Float%20%28single-precision%29))
  (|CallParentFunction DeltaSeconds) ; This node is disabled and will not be called.\nDrag off pins to build functionality.
)

(fn ConstructionScript
  (|CallParentFunction))

(fn ConfirmCamera
  (Utilities|IsValid (Variables|Default|GetSideCamera)
    (:Is%20Not%20Valid
      (bind _returnvalue (Game|SpawnActorfromClass "/Game/Blueprints/Battle/DemoCamera.DemoCamera_C" (Math|Transform|MakeTransform "0, 0,100.000000") "AlwaysSpawn" self 0))
      (Variables|Default|SetSideCamera _returnvalue))))