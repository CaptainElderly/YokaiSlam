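; Base game mode for sumo battles of up to eight slots, running rounds until the game state reports the match over.
; On play it fills empty character picks randomly, then each round resets the level, spawns and possesses fighters, and starts after a countdown.
; CheckStatus awards a point to the last non-disqualified Sumo, triggering the next round or a menu exit with reward or winner message.
; Several functions are empty stubs, and online matches add start delays.
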(event Custom|MatchExit
  (bind _returnvalue (CallFunction|GetSumoGameState))
  (if (Default|IsSingleplayer _returnvalue)
    (if (Default|IsLocalPlayerWinner _returnvalue)
      (CallFunction|GameExitWin)
      (else
        (Variables|/Game/Blueprints/Base/SumoGameInstance.SumoGameInstance_C|SetWinMessage (CallFunction|GetSumoGameInstance) (Utilities|Text|FormatText "{winner} Wins!" (Variables|/Game/Blueprints/Battle/Sumo.Sumo_C|GetCharacterName (Default|GetPlayerbyID _returnvalue (Variables|/Game/Blueprints/Battle/SumoGameState.SumoGameState_C|GetWinner _returnvalue)))) :!label _label)
        (CallFunction|GameExitGeneric)))
    (else
      (goto _label))))

(event Custom|StartRound
  (bind _returnvalue (CallFunction|GetSumoGameState))
  (bind _returnvalue_2 (Math|Float|MakeLiteralFloat 5.0))
  (Class|GameModeBase|ResetLevel)
  (Variables|/Game/Blueprints/Battle/SumoGameState.SumoGameState_C|SetGameStatus _returnvalue "NewEnumerator3")
  (if (CallFunction|IsOnline (Variables|/Game/Blueprints/Battle/SumoGameState.SumoGameState_C|GetActiveMatchInfo _returnvalue))
    (Utilities|FlowControl|Delay 3.0))
  (CallFunction|SpawnFighters)
  (Variables|/Game/Blueprints/Battle/SumoGameState.SumoGameState_C|SetStartTime _returnvalue (+ (GameState|GetServerWorldTimeSeconds (CallFunction|GetSumoGameState)) _returnvalue_2))
  (Utilities|FlowControl|Delay _returnvalue_2)
  (Variables|/Game/Blueprints/Battle/SumoGameState.SumoGameState_C|SetGameStatus _returnvalue "NewEnumerator0"))

(event Custom|CheckStatus
  (CallFunction|DetermineGameState))

(event Custom|RoundFinished
  (if (CallFunction|ShouldPlaySounds)
    (Audio|PlaySound2D "/Game/SFX/gong.gong" 0.2 1.3 0.0 0 0))
  (if (Default|IsGameOver (CallFunction|GetSumoGameState))
    (CallFunction|OnMatchEnded)
    (else
      (Utilities|FlowControl|Delay 4.0)
      (CallFunction|StartRound))))

(event Custom|BeginMatch
  (CallFunction|StartRound))

(event Custom|ManageAISelections
  (bind _returnvalue (CallFunction|GetSumoGameState))
  (bind _returnvalue_2 (CallFunction|GetSumoGameInstance))
  (bind _activematchinfo (Variables|/Game/Blueprints/Battle/SumoGameState.SumoGameState_C|GetActiveMatchInfo _returnvalue))
  ;[1 1 1] Default gamemode functionality uses this event as a fallback function. Any slots lacking a character choice are auto-filled with a random choice.
  (for _index (range 0 7)
    (if (and (Utilities|Enum|NotEqual(Enum) (CallFunction|GetPlayerTypeinSlot _activematchinfo _index) "NewEnumerator0") (not (CallFunction|HasCharacter _activematchinfo _index)))
      (CallFunction|SetCharacter _activematchinfo _index (Utilities|Struct|MakeCharacterSelection (Default|GetRandomCharacter _returnvalue_2 true) (select (Default|AreSkinsUnlocked _returnvalue_2) (Math|Random|RandomInteger 2) 0))))))

(event Custom|OnMatchEnded
  (if (CallFunction|ShouldPlaySounds)
    (Audio|PlaySound2D "/Game/SFX/yoooo.yoooo" 1.0 1.0 0.0 0 0))
  (Utilities|FlowControl|Delay 4.0)
  (CallFunction|MatchExit))

(event EventBeginPlay
  (CameraFades|StartCameraFade :self (Game|GetPlayerCameraManager 0) :FromAlpha 1.0 :Duration 1.0 :bHoldWhenFinished true)
  (Utilities|FlowControl|Delay 0.0)
  (CallFunction|ConfirmCamera)
  (CallFunction|ManageAISelections)
  (if (.ReturnValue (CallFunction|IsOnlineServer))
    (Utilities|FlowControl|Delay 3.0))
  (CallFunction|BeginMatch))

(event EventTick
  (params (DeltaSeconds :type Float%20%28single-precision%29))
  (CallFunction|ConfirmCamera))

(fn ConstructionScript)

(fn GetCenterOfGame
  (bind _positions (LocalVariables|GetPositions))
  (bind _outactors (Actor|GetAllActorsOfClass "/Game/Blueprints/Battle/Sumo.Sumo_C"))
  (if (|Aretheresumosatall? _outactors)
    (for _array_element _outactors
      (Utilities|Array|Add _positions (Transformation|GetActorLocation _array_element)))
    (return (Math|Vector|GetVectorArrayAverage _positions))))

(fn DetermineGameState
  (bind _returnvalue (CallFunction|GetSumoGameState))
  (if (Utilities|Enum|Equal(Enum) (CallFunction|GetMatchStatus) "NewEnumerator0")
    (bind _outactors (Actor|GetAllActorsOfClass "/Game/Blueprints/Battle/Sumo.Sumo_C"))
    (for _array_element _outactors
      (if (not (Variables|/Game/Blueprints/Battle/Sumo.Sumo_C|GetDisqualified _array_element))
        (Math|Integer|IncrementInt (LocalVariables|GetPlayersAlive)
          (:%20%20
            (LocalVariables|SetLastPlayerFoundAlive _array_element)))))
    (if (== (LocalVariables|GetPlayersAlive) 1)
      (Utilities|IsValid (LocalVariables|GetLastPlayerFoundAlive)
        (:Is%20Valid
          (Variables|/Game/Blueprints/Battle/SumoGameState.SumoGameState_C|SetGameStatus _returnvalue "NewEnumerator4")
          (Default|AddPoint _returnvalue (Variables|/Game/Blueprints/Battle/Sumo.Sumo_C|GetGameID (LocalVariables|GetLastPlayerFoundAlive)))
          (Variables|/Game/Blueprints/Battle/SumoGameState.SumoGameState_C|SetWinner _returnvalue (Variables|/Game/Blueprints/Battle/Sumo.Sumo_C|GetGameID (LocalVariables|GetLastPlayerFoundAlive)))
          (CallFunction|RoundFinished))))))

(fn SpawnFighters
  (bind _returnvalue (CallFunction|GetSumoGameState))
  (bind _activematchinfo (Variables|/Game/Blueprints/Battle/SumoGameState.SumoGameState_C|GetActiveMatchInfo _returnvalue))
  (for _index (range 0 7)
    (if (CallFunction|HasPlayer _activematchinfo _index)
      (Utilities|IsValid (Default|GetPlayerbyID (CallFunction|GetSumoGameState) _index)
        (:Is%20Not%20Valid
          (bind _returnvalue_2 (Game|SpawnActorfromClass (select (Utilities|IsValidClass (.Character (Utilities|Struct|BreakCharacterSelection (CallFunction|GetCharacter _activematchinfo _index)))) (.Character (Utilities|Struct|BreakCharacterSelection (CallFunction|GetCharacter _activematchinfo _index))) (Default|GetRandomCharacter (CallFunction|GetSumoGameInstance) true)) (Utilities|Array|Get(acopy) (Variables|Default|GetSpawnTransforms) _index) "AlwaysSpawn" 0 _index 0))
          (Utilities|Array|SetArrayElem (Variables|/Game/Blueprints/Battle/SumoGameState.SumoGameState_C|GetPlayers (CallFunction|GetSumoGameState)) _index _returnvalue_2 true)
          (switch Utilities|FlowControl|Switch|SwitchonPlayerType (CallFunction|GetPlayerTypeinSlot _activematchinfo _index)
            (:NewEnumerator1
              (Utilities|IsValid (Game|GetPlayerController _index) :!label _label
                (:Is%20Valid
                  (Pawn|Possess (Game|GetPlayerController _index) _returnvalue_2))))
            (:NewEnumerator4
              (goto _label))
            (:NewEnumerator2
              (Pawn|SpawnDefaultController _returnvalue_2 :!label _label_2))
            (:NewEnumerator3
              (goto _label_2))))))))

(fn GetCharacterfromSlot)

(fn UnlockEnemyCharacter
  (params (Slot :type Integer)))

(fn ConfirmCamera)

(fn GameExitLose
  (Default|EnterMenu (CallFunction|GetSumoGameInstance) "/Game/Blueprints/Menu/FailureMenu.FailureMenu_C" 3.0 false false true))

(fn LocalPlayerIsLoser
  (bind _returnvalue (CallFunction|GetSumoGameState))
  (bind _winner (Variables|/Game/Blueprints/Battle/SumoGameState.SumoGameState_C|GetWinner _returnvalue))
  (if (!= _winner 0)
    (return (not (Pawn|IsLocalPlayerController (Pawn|GetController (Default|GetPlayerbyID _returnvalue _winner)))))))

(fn GameExitWin
  (bind _returnvalue (CallFunction|GetSumoGameInstance))
  (CallFunction|GiveMatchReward (Variables|/Game/Blueprints/Base/SumoGameInstance.SumoGameInstance_C|GetPlannedMatch _returnvalue))
  (Default|EnterMenu _returnvalue "/Game/Blueprints/Menu/WinMenu.WinMenu_C" 3.0 false false true))

(fn GameExitStandings
  (Default|EnterMenu (CallFunction|GetSumoGameInstance) "/Game/Blueprints/Menu/StandingsHud.StandingsHud_C" 3.0 false false true))

(fn GameExitGeneric
  (Default|EnterMenu (CallFunction|GetSumoGameInstance) "/Game/Blueprints/Menu/GenericMessageMenu.GenericMessageMenu_C" 3.0 false true true))

(fn ShouldPlaySounds
  (return true))

(fn SpawnCoinRenderer
  (bind _outactors (Actor|GetAllActorsOfClass "/Game/Blueprints/CoinCapture.CoinCapture_C"))
  (if (== (Utilities|Array|Length _outactors) 0)
    (Game|SpawnActorfromClass "/Game/Blueprints/CoinCapture.CoinCapture_C" (Math|Transform|MakeTransform "0, 0,50000.000000") "AlwaysSpawn" self 0)))