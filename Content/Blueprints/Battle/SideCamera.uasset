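; Side-view battle camera actor that keeps the Sumo fighters framed.
; Each tick it snaps to the averaged Sumo position at a fixed height and scales its spring arm with the distance between the first two Sumos.
; It eases its yaw perpendicular to the line between left and right fighters.
; Player 1 is treated as left and player 2 as right, falling back to other Sumo actors in the level.
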(event EventBeginPlay
  (Transformation|SetActorLocation (CallFunction|GetTargetPos) false false)
  (Transformation|SetActorRotation (CallFunction|GetTargetAngle)))

(event Collision|EventActorBeginOverlap
  (params (OtherActor :type Actor%20Object%20Reference)))

(event EventTick
  (params (DeltaSeconds :type Float%20%28single-precision%29))
  (Transformation|SetActorLocation (CallFunction|GetTargetPos) false false)
  (Transformation|SetActorRotation (Math|Interpolation|RInterpTo (Transformation|GetActorRotation) (CallFunction|GetTargetAngle) DeltaSeconds 1.0))
  (Variables|/Script/Engine.SpringArmComponent|SetTargetArmLength (Variables|Default|GetSpringArm) (CallFunction|GetCameraDistance)))

(fn ConstructionScript)

(fn GetTargetPos
  (bind _outactors (Actor|GetAllActorsOfClass "/Game/Blueprints/Battle/Sumo.Sumo_C"))
  (for _array_element _outactors
    (LocalVariables|SetFocusPos (+ (* (+ (LocalVariables|GetFocusPos) (/ (Transformation|GetActorLocation _array_element) (Utilities|Array|Length _outactors))) "1.000000,1.000000, 0") "0, 0,70.000000")))
  (return (LocalVariables|GetFocusPos)))

(fn GetTargetAngle
  (bind _returnvalue (CallFunction|GetLeftCharacter))
  (bind _returnvalue_2 (CallFunction|GetRightCharacter))
  (Utilities|IsValid _returnvalue
    (:Is%20Valid
      (Utilities|IsValid _returnvalue_2
        (:Is%20Valid
          (return (CallFunction|RotationfromTwoPawns _returnvalue _returnvalue_2)))
        (:Is%20Not%20Valid
          _)))
    (:Is%20Not%20Valid
      _))
  (return "0, 0, 0"))

(fn GetCameraDistance
  (bind _outactors (Actor|GetAllActorsOfClass "/Game/Blueprints/Battle/Sumo.Sumo_C"))
  (if (> (Utilities|Array|Length _outactors) 1)
    (if (and (Utilities|IsValid (Utilities|Array|Get(acopy) _outactors)) (Utilities|IsValid (Utilities|Array|Get(acopy) _outactors 1)))
      (return (Math|Float|Max(Float) (* (Math|Vector|Distance2D(Vector) (Transformation|GetActorLocation (Utilities|Array|Get(acopy) _outactors)) (Transformation|GetActorLocation (Utilities|Array|Get(acopy) _outactors 1))) 1.3) 2e+02))
      (else
        _)))
  (return 3e+02))

(fn RotationfromTwoPawns
  (params (Left :type Pawn%20Object%20Reference) (Right :type Pawn%20Object%20Reference))
  (return (Math|Rotator|MakeRotfromZX (Math|Vector|MakeVector 0.0 0.0 1.0) (Math|Vector|GetRightVector (Math|Rotator|FindLookatRotation (Transformation|GetActorLocation Right) (Transformation|GetActorLocation Left))))))

(fn GetLeftCharacter
  (bind _returnvalue (Game|Player|GetPlayerPawn 0))
  (Utilities|IsValid _returnvalue
    (:Is%20Valid
      (bind _assumo (Utilities|Casting|CastToSumo _returnvalue)
        (:then
          (return _assumo))
        (:CastFailed
          _)))
    (:Is%20Not%20Valid
      _))
  (bind _outactors (Actor|GetAllActorsOfClass "/Game/Blueprints/Battle/Sumo.Sumo_C"))
  (if (Utilities|Array|IsValidIndex _outactors)
    (return (Utilities|Array|Get(acopy) _outactors))))

(fn GetRightCharacter
  (bind _returnvalue (Game|Player|GetPlayerPawn 1))
  (Utilities|IsValid _returnvalue
    (:Is%20Valid
      (bind _assumo (Utilities|Casting|CastToSumo _returnvalue)
        (:then
          (return _assumo))
        (:CastFailed
          _)))
    (:Is%20Not%20Valid
      _))
  (bind _outactors (Actor|GetAllActorsOfClass "/Game/Blueprints/Battle/Sumo.Sumo_C"))
  (for _array_element _outactors
    (if (!= _array_element (CallFunction|GetLeftCharacter))
      (return _array_element))))

(fn CorrectedPlayerSides)