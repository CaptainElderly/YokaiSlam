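; Demo game mode for the sumo battle game that runs endless rounds with random characters, apparently as an attract mode.
; Each round fades in, randomizes character and skin (when skins are unlocked) for occupied slots, resets the level and spawns fighters; round end fades out and restarts.
; Overrides report no points, never game over and no sounds, add a demo HUD, and spawn a demo camera if none is valid.
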(event EventBeginPlay
  (|CallParentFunction) ; This node is disabled and will not be called.\nDrag off pins to build functionality.
)

(event EventTick
  (params (DeltaSeconds :type Float%20%28single-precision%29))
  (|CallParentFunction DeltaSeconds) ; This node is disabled and will not be called.\nDrag off pins to build functionality.
)

(event EventStartRound
  (CallFunction|ManageAISelections)
  (CameraFades|StartCameraFade (Game|GetPlayerCameraManager 0) 1.0 0.0 0.5 "(R=0.000000,G=0.000000,B=0.000000,A=1.000000)" false true)
  (Class|GameModeBase|ResetLevel)
  (CallFunction|SpawnFighters)
  (Variables|/Game/Blueprints/Battle/SumoGameState.SumoGameState_C|SetGameStatus (CallFunction|GetSumoGameState) "NewEnumerator0"))

(event EventRoundFinished
  (Utilities|FlowControl|Delay 2.0)
  (CameraFades|StartCameraFade (Game|GetPlayerCameraManager 0) 0.0 1.0 0.4 "(R=0.000000,G=0.000000,B=0.000000,A=1.000000)" false true)
  (Utilities|FlowControl|Delay 0.5)
  (CallFunction|StartRound))

(event EventManageAISelections
  (bind _returnvalue (CallFunction|GetSumoGameInstance))
  (bind _returnvalue_2 (CallFunction|GetSumoGameState))
  (bind _activematchinfo (Variables|/Game/Blueprints/Battle/SumoGameState.SumoGameState_C|GetActiveMatchInfo _returnvalue_2))
  (for _index (range 0 8)
    (if (CallFunction|HasPlayer _activematchinfo _index)
      (CallFunction|SetCharacter _activematchinfo _index (Utilities|Struct|MakeCharacterSelection (Default|GetRandomCharacter _returnvalue true) (select (Default|AreSkinsUnlocked _returnvalue) (Math|Random|RandomInteger 2) 0))))))

(fn ConstructionScript
  (|CallParentFunction))

(fn GetPlayerPoints
  (params (GameID :type Integer))
  (return 0))

(fn IsGameOver
  (return false))

(fn ShouldPlaySounds
  (return false))

(fn SpawnHUD
  (bind _returnvalue (UserInterface|CreateWidget "/Game/Blueprints/HUD/DemoHUD.DemoHUD_C" (Game|GetPlayerController 0)))
  (UserInterface|Viewport|AddtoViewport _returnvalue 0))

(fn ConfirmCamera
  (Utilities|IsValid (Variables|Default|GetSideCamera)
    (:Is%20Not%20Valid
      (bind _returnvalue (Game|SpawnActorfromClass "/Game/Blueprints/Battle/DemoCamera.DemoCamera_C" (Math|Transform|MakeTransform "0, 0,100.000000") "AlwaysSpawn" self 0))
      (Variables|Default|SetSideCamera _returnvalue)
      (bind _outactors (Actor|GetAllActorsOfClass "/Script/Engine.PlayerController"))
      (for _array_element _outactors
        _))))