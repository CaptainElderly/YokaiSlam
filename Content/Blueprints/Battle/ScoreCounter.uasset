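; ScoreCounter is a battle actor that displays one player's Sumo score, identified by GameID, as a physical coin stack.
; Tick polls the Sumo game state and calls Rebuild when the score changes, with an initial build shortly after BeginPlay.
; Rebuild tints the plane's dynamic material with a darkened player color, then adds or destroys coin meshes to match the score, up to ten, with random offset and yaw.
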(event EventBeginPlay
  (Utilities|FlowControl|Delay 0.2)
  (CallFunction|Rebuild))

(event Collision|EventActorBeginOverlap
  (params (OtherActor :type Actor%20Object%20Reference)))

(event EventTick
  (params (DeltaSeconds :type Float%20%28single-precision%29))
  (bind _returnvalue (CallFunction|GetSumoGameState))
  (bind _gameid (Variables|Default|GetGameID))
  (bind _returnvalue_2 (Default|GetPlayerScore _returnvalue _gameid))
  (if (!= (Variables|Default|GetCurrentScore) _returnvalue_2)
    (Variables|Default|SetCurrentScore _returnvalue_2)
    (CallFunction|Rebuild)))

(fn ConstructionScript)

(fn Rebuild
  (bind _plane (Variables|Default|GetPlane))
  (bind _coinstack (Variables|Default|GetCoinStack))
  (bind _returnvalue (Rendering|Material|GetMaterial _plane 0))
  (Utilities|IsValid _returnvalue
    (:Is%20Valid
      (Utilities|Casting|CastToMaterialInstanceDynamic _returnvalue
        (:then
          _)
        (:CastFailed
          (bind _returnvalue_2 (Rendering|Material|CreateDynamicMaterialInstance _plane 0 _returnvalue "None" :!class /Script/Engine.PrimitiveComponent))
          (Rendering|Material|SetMaterial _plane 0 _returnvalue_2)))
      (bind _asmaterial_instance_dynamic (Utilities|Casting|CastToMaterialInstanceDynamic _returnvalue))
      (Rendering|Material|SetVectorParameterValue _asmaterial_instance_dynamic "Color" (* (Default|GetPlayerColor (CallFunction|GetSumoGameInstance) (Variables|Default|GetGameID)) "(R=0.250000,G=0.250000,B=0.250000,A=1.000000)") :!class /Script/Engine.MaterialInstanceDynamic)
      (for _index (range 1 10)
        (if (>= (Variables|Default|GetCurrentScore) _index)
          (if (Utilities|Array|IsValidIndex _coinstack _index)
            (Utilities|IsValid (Utilities|Array|Get(acopy) _coinstack _index)
              (:Is%20Not%20Valid
                _)))
          (bind _returnvalue_3 (AddComponent|AddStaticMeshComponent false (Math|Transform|MakeTransform (+ (* (Math|Random|RandomUnitVector) "3.000000,3.000000,0.000000") (Math|Vector|MakeVector 0.0 0.0 (+ (* (Math|Conversions|ToFloat(Integer) _index) 0.9) -0.45))) (Math|Rotator|MakeRotator 0.0 0.0 (Math|Random|RandomFloatinRange 0.0 3.6e+02)) "5.000000,5.000000,5.000000")))
          (Transformation|AttachComponentToComponent _returnvalue_3 (Variables|Default|GetScene) "None" "KeepRelative" "KeepRelative" "KeepRelative" false)
          (Utilities|Array|SetArrayElem _coinstack _index _returnvalue_3 true)
          (elif (Utilities|Array|IsValidIndex _coinstack _index)
            (Utilities|IsValid (Utilities|Array|Get(acopy) _coinstack _index)
              (:Is%20Valid
                (Components|DestroyComponent (Utilities|Array|Get(acopy) _coinstack _index))))))))))