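; Demo camera for the Sumo battle game that holds a fixed point just above the world origin and slowly pans in a full circle.
; Each tick it reapplies that position and interpolates rotation toward a yaw derived from game time, after snapping to both on BeginPlay.
; Helpers that find left and right Sumo characters and compute a side-on rotation between two pawns are defined but not used by this movement.
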(event EventBeginPlay
  (Transformation|SetActorLocation (CallFunction|GetTargetPos) false false)
  (Transformation|SetActorRotation (CallFunction|GetTargetAngle)))

(event Collision|EventActorBeginOverlap
  (params (OtherActor :type Actor%20Object%20Reference)))

(event EventTick
  (params (DeltaSeconds :type Float%20%28single-precision%29))
  (Transformation|SetActorLocation (CallFunction|GetTargetPos) false false)
  (Transformation|SetActorRotation (Math|Interpolation|RInterpTo (Transformation|GetActorRotation) (CallFunction|GetTargetAngle) DeltaSeconds 2.0)))

(fn ConstructionScript)

(fn GetTargetPos
  (return "0, 0,70.000000"))

(fn GetTargetAngle
  (return (Math|Rotator|MakeRotator 0.0 0.0 (* (Utilities|Time|GetGameTimeinSeconds) 15.0))))

(fn RotationfromTwoPawns
  (params (Left :type Pawn%20Object%20Reference) (Right :type Pawn%20Object%20Reference))
  (return (Math|Rotator|MakeRotfromZX (Math|Vector|MakeVector 0.0 0.0 1.0) (Math|Vector|GetRightVector (Math|Rotator|FindLookatRotation (Transformation|GetActorLocation Right) (Transformation|GetActorLocation Left))))))

(fn GetLeftCharacter
  (bind _returnvalue (Game|Player|GetPlayerPawn 0))
  (Utilities|IsValid _returnvalue
    (:Is%20Valid
      (bind _assumo (Utilities|Casting|CastToSumo _returnvalue)
        (:then
          (return _assumo))
        (:CastFailed
          _)))
    (:Is%20Not%20Valid
      _))
  (bind _outactors (Actor|GetAllActorsOfClass "/Game/Blueprints/Battle/Sumo.Sumo_C"))
  (return (Utilities|Array|Get(acopy) _outactors)))

(fn GetRightCharacter
  (bind _returnvalue (Game|Player|GetPlayerPawn 1))
  (Utilities|IsValid _returnvalue
    (:Is%20Valid
      (bind _assumo (Utilities|Casting|CastToSumo _returnvalue)
        (:then
          (return _assumo))
        (:CastFailed
          _)))
    (:Is%20Not%20Valid
      _))
  (bind _outactors (Actor|GetAllActorsOfClass "/Game/Blueprints/Battle/Sumo.Sumo_C"))
  (for _array_element _outactors
    (if (!= _array_element (CallFunction|GetLeftCharacter))
      (return _array_element))))