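; Battle audience member, a Kappa spectator that carries the flags of the two fighters and can be squashed by a Sumo.
; Construction randomizes mesh offset, yaw, scale and body material, including rare variants.
; After a zero-length delay on BeginPlay, it reads both match characters' class defaults to apply their flag materials.
; A Sumo hit flattens it, clears its animation class, disables collision and plays a squeak.
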(event OnComponentHit(Box)
  (params (HitComponent :type Primitive%20Component%20Object%20Reference) (OtherActor :type Actor%20Object%20Reference) (OtherComp :type Primitive%20Component%20Object%20Reference) (NormalImpulse :type Vector :default "0, 0, 0") (Hit :type Hit%20Result%20Structure%20%28by%20ref%29))
  (Utilities|Casting|CastToSumo OtherActor)
  (CallFunction|Squash))

(event Custom|Squash
  (bind _scene (Variables|Default|GetScene))
  (Transformation|SetRelativeRotation _scene "90.000000,0.000000,0.000000" false false)
  (Transformation|SetRelativeLocation _scene "0, 0,-30.000000" false false)
  (Transformation|SetRelativeScale3D _scene "0.100000,1.000000,1.000000")
  (Class|SkeletalMeshComponent|SetAnimClass (Variables|Default|GetSkeletalMesh))
  (Collision|SetCollisionEnabled (Variables|Default|GetBox) "NoCollision")
  (Audio|PlaySoundatLocation "/Game/SFX/squeak_Cue.squeak_Cue" (Transformation|GetActorLocation) "0, 0, 0" 1.0 1.0 0.0 0 0 0))

(event EventBeginPlay
  (Utilities|FlowControl|Delay 0.0)
  (CallFunction|SetupFlags))

(event Collision|EventActorBeginOverlap
  (params (OtherActor :type Actor%20Object%20Reference)))

(event EventTick
  (params (DeltaSeconds :type Float%20%28single-precision%29)))

(fn ConstructionScript
  (bind _skeletalmesh (Variables|Default|GetSkeletalMesh))
  (Transformation|SetRelativeTransform (Variables|Default|GetSkeletalMesh) (Math|Transform|MakeTransform (* (Math|Random|RandomUnitVector) "5.000000,5.000000,0.000000") (Math|Rotator|MakeRotator 0.0 0.0 (Math|Random|RandomFloatinRange -15.0 15.0)) (Math|Conversions|ToVector(Float) (* (Math|Random|RandomFloatinRange 0.9 1.1) 6.0))) false false)
  (if (Math|Random|RandomBool)
    (Rendering|Material|SetMaterial _skeletalmesh 1 "/Game/Characters/Kappa/kappa2_material.kappa2_material")
    (if (== (Math|Random|RandomIntegerinRange 0 20) 0)
      (Rendering|Material|SetMaterial _skeletalmesh 1 "/Game/Characters/Kappa/kappa3_material.kappa3_material")
      (elif (== (Math|Random|RandomIntegerinRange 0 12) 0)
        (Rendering|Material|SetMaterial _skeletalmesh 1 "/Game/Characters/Kappa/kappa_fucker_material.kappa_fucker_material")))))

(fn SetupFlags
  (bind _returnvalue (CallFunction|GetSumoGameState))
  (bind _skeletalmesh (Variables|Default|GetSkeletalMesh))
  (bind _activematchinfo (Variables|/Game/Blueprints/Battle/SumoGameState.SumoGameState_C|GetActiveMatchInfo _returnvalue))
  (bind _returnvalue_2 (CallFunction|GetCharacter _activematchinfo 1))
  (bind _returnvalue_3 (CallFunction|GetCharacter _activematchinfo))
  (bind _character (Utilities|Struct|BreakCharacterSelection _returnvalue_2))
  (bind _character_2 (Utilities|Struct|BreakCharacterSelection _returnvalue_3))
  (bind _flag (Utilities|GetClassDefaults _character))
  (bind _flag_2 (Utilities|GetClassDefaults _character_2))
  (Utilities|IsValid _returnvalue
    (:Is%20Valid
      (Utilities|FlowControl|Sequence
        (:then_0
          (if (Utilities|IsValidClass _character_2)
            (Utilities|IsValid _flag_2
              (:Is%20Valid
                (Rendering|Material|SetMaterial _skeletalmesh 0 _flag_2)))))
        (:then_1
          (if (Utilities|IsValidClass _character)
            (Utilities|IsValid _flag
              (:Is%20Valid
                (Rendering|Material|SetMaterial _skeletalmesh 2 _flag)))))
        (:then_2
          (return))))))