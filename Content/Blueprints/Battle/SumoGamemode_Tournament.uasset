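; Tournament game mode for sumo battles that runs the player through a queue of opponents.
; AI selection fills character slot 1 of the active match from the tournament queue at the current progress index, if that index is valid.
; On match exit, a loss takes the lose exit; otherwise it calls ProceedTournament on the game instance's planned match, taking the win exit on true and standings on false.
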(event EventTick
  (params (DeltaSeconds :type Float%20%28single-precision%29))
  (|CallParentFunction DeltaSeconds) ; This node is disabled and will not be called.\nDrag off pins to build functionality.
)

(event EventManageAISelections
  (bind _returnvalue (CallFunction|GetSumoGameState))
  (bind _activematchinfo (Variables|/Game/Blueprints/Battle/SumoGameState.SumoGameState_C|GetActiveMatchInfo _returnvalue))
  (bind (_players _characters _targetmap _targetgamemode _tournamentqueue _tournamentprogress) (Utilities|Struct|BreakMatchSettings _activematchinfo))
  (if (Utilities|Array|IsValidIndex _tournamentqueue _tournamentprogress)
    (CallFunction|SetCharacter _activematchinfo 1 (Utilities|Array|Get(acopy) _tournamentqueue _tournamentprogress))))

(event EventMatchExit
  ;[1 1 1] We won the game! Let's proceed to the next opponent if there is one!
  (if (CallFunction|LocalPlayerIsLoser)
    (CallFunction|GameExitLose)
    (else
      (bind _complete (CallFunction|ProceedTournament (Variables|/Game/Blueprints/Base/SumoGameInstance.SumoGameInstance_C|GetPlannedMatch (CallFunction|GetSumoGameInstance))))
      (if _complete
        (CallFunction|GameExitWin)
        (else
          (CallFunction|GameExitStandings))))))

(fn ConstructionScript
  (|CallParentFunction))