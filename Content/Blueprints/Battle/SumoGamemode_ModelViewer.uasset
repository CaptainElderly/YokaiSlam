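; Sumo game mode variant for the model viewer, with a simplified round flow.
; StartRound resets the level, spawns the fighters and sets the game state's status directly, while RoundFinished does nothing.
; MovementRulesActive returns true only when the current level is VoidArena or TournamentArena.
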(event EventBeginPlay
  (|CallParentFunction) ; This node is disabled and will not be called.\nDrag off pins to build functionality.
)

(event EventTick
  (params (DeltaSeconds :type Float%20%28single-precision%29))
  (|CallParentFunction DeltaSeconds) ; This node is disabled and will not be called.\nDrag off pins to build functionality.
)

(event EventStartRound
  (Class|GameModeBase|ResetLevel)
  (CallFunction|SpawnFighters)
  (Variables|/Game/Blueprints/Battle/SumoGameState.SumoGameState_C|SetGameStatus (CallFunction|GetSumoGameState) "NewEnumerator0"))

(event EventRoundFinished)

(fn ConstructionScript
  (|CallParentFunction))

(fn MovementRulesActive
  (bind _returnvalue (Game|GetCurrentLevelName true))
  (return (or (Utilities|Name|Equal(Name) (Utilities|String|StringToName _returnvalue) "VoidArena") (Utilities|Name|Equal(Name) (Utilities|String|StringToName _returnvalue) "TournamentArena"))))