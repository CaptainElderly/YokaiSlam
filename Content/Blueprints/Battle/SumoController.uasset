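; Player controller for sumo battles, handling HUD, camera and menu input.
; On possess and begin play it creates a battle or demo HUD for the first player and sets game-only input.
; It keeps the view on the game state's side camera, re-checking every tick.
; Pause input opens the pause menu outside demo mode, while any key in the demo gamemode returns to the main menu.
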(event Custom|DestroyMenu
  (Widget|RemovefromParent (Variables|/Game/Blueprints/Base/SumoBasePlayerController.SumoBasePlayerController_C|GetCurrentMenu (CallFunction|GetMasterController))))

(event EventBeginPlay
  (bind _returnvalue (CallFunction|GetSumoGameState))
  (bind _sidecamera (Variables|/Game/Blueprints/Battle/SumoGameState.SumoGameState_C|GetSideCamera _returnvalue))
  (CallFunction|CreateHUD)
  (Input|SetInputModeGameOnly self)
  (if (!= (Pawn|GetViewTarget) _sidecamera)
    (Game|Player|SetViewTargetwithBlend self _sidecamera 0.0 "VTBlend_Cubic" 0.0 false)))

(event EventTick
  (params (DeltaSeconds :type Float%20%28single-precision%29))
  (bind _returnvalue (CallFunction|GetSumoGameState))
  (bind _sidecamera (Variables|/Game/Blueprints/Battle/SumoGameState.SumoGameState_C|GetSideCamera _returnvalue))
  (|CallParentFunction DeltaSeconds)
  (CallFunction|UpdateEpicMode)
  (if (!= (Pawn|GetViewTarget) _sidecamera)
    (Game|Player|SetViewTargetwithBlend self _sidecamera 0.0 "VTBlend_Cubic" 0.0 false)))

(event EventPossess
  (params (PossessedPawn :type Pawn%20Object%20Reference))
  (bind _returnvalue (CallFunction|GetSumoGameState))
  (bind _sidecamera (Variables|/Game/Blueprints/Battle/SumoGameState.SumoGameState_C|GetSideCamera _returnvalue))
  (CallFunction|CreateHUD)
  (Input|SetInputModeGameOnly self)
  (if (!= (Pawn|GetViewTarget) _sidecamera)
    (Game|Player|SetViewTargetwithBlend self _sidecamera 0.0 "VTBlend_Cubic" 0.0 false)))

(event Input|ActionEvents|InputActionPause
  (params (Key :type Key%20Structure :default "None"))
  (:Pressed
    (Utilities|SkipifDemoMode)
    (Default|EnterMenu (CallFunction|GetSumoGameInstance) "/Game/Blueprints/Menu/PauseMenu.PauseMenu_C" 1.0 true false true)))

(event Input|KeyboardEvents|P
  (params (Key :type Key%20Structure :default "None"))
  (:Pressed
    (Utilities|SkipifDemoMode)
    (Default|EnterMenu (CallFunction|GetSumoGameInstance) "/Game/Blueprints/Menu/PauseMenu.PauseMenu_C" 1.0 true false true)))

(event Input|KeyboardEvents|AnyKey
  (params (Key :type Key%20Structure :default "None"))
  (:Pressed
    (Utilities|Casting|CastToSumoGamemode_Demo (CallFunction|GetSumoGamemode))
    (if (not (Variables|Default|GetLeavingDemo))
      (Default|EnterMenu (CallFunction|GetSumoGameInstance) "/Game/Blueprints/Menu/MainMenu.MainMenu_C" 1.0 false true false)
      (Variables|Default|SetLeavingDemo true))))

(fn ConstructionScript)

(fn UpdateEpicMode)

(fn CreateHUD
  (bind _returnvalue (Game|GetPlayerController 0))
  (if (== _returnvalue self)
    (Utilities|IsValid (Variables|Default|GetHUD)
      (:Is%20Not%20Valid
        (bind _returnvalue_2 (UserInterface|CreateWidget (select (Utilities|IsDemoMode) "/Game/Blueprints/HUD/DemoHUD.DemoHUD_C" "/Game/Blueprints/HUD/BattleHUD.BattleHUD_C") _returnvalue))
        (UserInterface|Viewport|AddtoViewport _returnvalue_2 0)
        (Variables|Default|SetHUD _returnvalue_2)))))